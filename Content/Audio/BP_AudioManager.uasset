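; Audio manager actor that plays menu music or in-game crowd ambience and drives the crowd's reaction to excitement.
; It creates music and crowd audio components on BeginPlay, leaving only one playing depending on IsMenu.
; Excitement maps to sitting, standing or cheering states; changes fire an audio trigger parameter and update CrowdController VFX.
; Crowd volume is either muted instantly or animated by a timeline.
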(event `UpdateCrowdVolume`
  (params (IsSilencing :type Boolean))
  (bind _crowdaudiocomponent (`self.CrowdAudioComponent`))
  (if IsSilencing
    (`AudioComponent.SetVolumeMultiplier` _crowdaudiocomponent 0.0)
    (else
      (bind (_direction _volume) (`Timeline|CrowdVolumeChange` :!via `PlayFromStart`)
        (:`Update`
          (`AudioComponent.SetVolumeMultiplier` _crowdaudiocomponent _volume))))))

(event `UnSilenceCrowd`)

(event `Update Crowd Cheering`
  (params (Excitement :type "Float (double-precision)"))
  (bind _state (`self.DetectState` Excitement))
  (if (not (== _state (`self.currentState`)))
    (set `self.currentState` _state)
    (`KismetSystemLibrary.PrintString` (`KismetStringLibrary.Conv_NameToString` _state))
    (message `AudioParameterControllerInterface.SetTriggerParameter` (`self.CrowdAudioComponent`) _state)
    (`/Game/BluePrints/GlorySystem/CrowdVFX/BP_VFXCrowdController.Change Crowd VFX` (`self.CrowdController`) _state)))

(event `CreateAudioComponents`
  (bind _returnvalue (`AddComponent|NODE_AddAudioComponent-0`))
  (set `self.CrowdAudioComponent` _returnvalue)
  (bind _returnvalue_2 (`AddComponent|NODE_AddAudioComponent-1`))
  (set `self.MusicAudioComponent` _returnvalue_2))

(event `PlayMusic`
  (`self.CreateAudioComponents`))

(event `self.ReceiveBeginPlay`
  (bind _musicaudiocomponent (`self.MusicAudioComponent`))
  (`self.PlayMusic`)
  (if (`self.isMenu`)
    (`AudioComponent.Play` _musicaudiocomponent 0.0)
    (`AudioComponent.Stop` (`self.CrowdAudioComponent`))
    (else
      (`AudioComponent.Play` _musicaudiocomponent 0.0)
      (`AudioComponent.Play` (`self.CrowdAudioComponent`) 0.0)
      (`AudioComponent.Stop` _musicaudiocomponent))))

(fn `DetectState`
  (params (Excitement :type "Float (double-precision)"))
  (returns (State :type Name))
  (locals (StateIndex :type Integer :default 0))
  (bind _stateindex (`local.StateIndex`))
  (set `local.StateIndex` (`KismetMathLibrary.FCeil` (- (/ (`KismetMathLibrary.FClamp` (* Excitement 4.0) 0.0 200.0) 99.0) 1.0)))
  (if (> 0 _stateindex)
    (set `local.StateIndex` 0))
  (return (select `int` _stateindex :`0` "State_Sitting" :`1` "State_Standing" :`2` "State_Cheering" :`3` "NULL" :!type "Name")))

(fn `UserConstructionScript`)