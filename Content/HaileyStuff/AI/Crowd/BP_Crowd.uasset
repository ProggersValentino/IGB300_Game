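; BP_Crowd is a crowd AI character that throws a ball once on BeginPlay.
; ThrowBall plays the aim montage, spawns an Interactable_Ball attached to the right-hand socket, then plays the throw montage, detaches the ball and applies a forward impulse scaled by ThrowForce.
; The sequence has no delays or anim notifies, so the ball is held and released in the same frame, with debug prints marking each stage.
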(event `self.ReceiveBeginPlay`
  (`self.ThrowBall`))

(fn `ThrowBall`
  (`KismetSystemLibrary.PrintString` "Holding")
  (`self.PlayAnimMontage` "/Game/HaileyStuff/AI/Animations/AM_Aim.AM_Aim" 1.0 "Default")
  (bind _returnvalue (`|SpawnActorFromClass` "/Game/HaileyStuff/Blueprints/Interactable_Ball.Interactable_Ball_C" (`SceneComponent.GetSocketTransform` (`self.Mesh`) "Ball_Socket_R" "RTS_World") "Undefined" "MultiplyWithRoot" null null))
  (bind _output_get (set `self.HeldItem` _returnvalue))
  (`PrimitiveComponent.SetCollisionEnabled` (`/Game/HaileyStuff/Blueprints/Interactable_Ball.Ball` (`self.HeldItem`)) "NoCollision")
  (`self.K2_AttachToComponent` _output_get (`self.Mesh`) "Ball_Socket_R" "SnapToTarget" "SnapToTarget" "KeepRelative" true)
  (`KismetSystemLibrary.PrintString` "released")
  (`self.PlayAnimMontage` "/Game/HaileyStuff/AI/Animations/AM_Throw.AM_Throw" 1.0 "Default")
  (`self.K2_DetachFromActor` (`self.HeldItem`) "KeepWorld" "KeepWorld" "KeepWorld")
  (`PrimitiveComponent.SetSimulatePhysics` (`/Game/HaileyStuff/Blueprints/Interactable_Ball.Ball` (`self.HeldItem`)) true)
  (`PrimitiveComponent.SetCollisionEnabled` (`/Game/HaileyStuff/Blueprints/Interactable_Ball.Ball` (`self.HeldItem`)) "QueryAndPhysics")
  (`PrimitiveComponent.AddImpulse` (`/Game/HaileyStuff/Blueprints/Interactable_Ball.Ball` (`self.HeldItem`)) (* (`self.GetActorForwardVector`) (`self.Throw Force`)) "None" false))

(fn `UserConstructionScript`)