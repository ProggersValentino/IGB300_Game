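; BP_Player_Stats tracks the player's XP and level and shows them on the HUD.
; On BeginPlay it waits one tick, finds the NewHUD actor, and fills its XP bar, XP text and level text.
; IncreaseXP adds XP and, at the cap, calls IncreaseLevel, then refreshes the XP display only in that branch.
; IncreaseLevel raises the level and XP cap, resets XP to zero and updates the level text.
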(event `self.ReceiveBeginPlay`
  (`KismetSystemLibrary.DelayUntilNextTick`)
  (bind _returnvalue (`GameplayStatics.GetActorOfClass` "/Game/HaileyStuff/UI/NewHUD.NewHUD_C"))
  (set `self.HUD` _returnvalue)
  (`ProgressBar.SetPercent` (`/Game/HaileyStuff/UI/Widget_HUD.XPBar` (`/Game/HaileyStuff/UI/NewHUD.UI_Ref` (`self.HUD`))) (/ (`self.XP`) (`self.Max XP`)))
  (`TextBlock.SetText` (`/Game/HaileyStuff/UI/Widget_HUD.XPTxt` (`/Game/HaileyStuff/UI/NewHUD.UI_Ref` (`self.HUD`))) (`|FormatText` "{Current XP} / {Max XP}" (`self.XP`) (`self.Max XP`)))
  (`TextBlock.SetText` (`/Game/HaileyStuff/UI/Widget_HUD.LevelTxt` (`/Game/HaileyStuff/UI/NewHUD.UI_Ref` (`self.HUD`))) (`KismetTextLibrary.Conv_IntToText` (`self.Level`))))

(fn `Increase Level`
  (params (`Added Level` :type Integer))
  (set `self.Level` (+ (`self.Level`) `Added Level`))
  (set `self.Max XP` (+ (`self.Max XP`) 150.0))
  (set `self.XP` 0.0)
  (`TextBlock.SetText` (`/Game/HaileyStuff/UI/Widget_HUD.LevelTxt` (`/Game/HaileyStuff/UI/NewHUD.UI_Ref` (`self.HUD`))) (`KismetTextLibrary.Conv_IntToText` (`self.Level`))))

(fn `Increase XP`
  (params (`Added XP` :type "Float (double-precision)"))
  (set `self.XP` (+ (`self.XP`) `Added XP`))
  (if (>= (`self.XP`) (`self.Max XP`))
    (`self.Increase Level` 1)
    (`ProgressBar.SetPercent` (`/Game/HaileyStuff/UI/Widget_HUD.XPBar` (`/Game/HaileyStuff/UI/NewHUD.UI_Ref` (`self.HUD`))) (/ (`self.XP`) (`self.Max XP`)))
    (`TextBlock.SetText` (`/Game/HaileyStuff/UI/Widget_HUD.XPTxt` (`/Game/HaileyStuff/UI/NewHUD.UI_Ref` (`self.HUD`))) (`|FormatText` "{Current XP} / {Max XP}" (`self.XP`) (`self.Max XP`)))))

(fn `UserConstructionScript`)