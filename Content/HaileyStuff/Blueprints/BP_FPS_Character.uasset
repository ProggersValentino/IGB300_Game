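; First-person player character with mouse look, jumping, interaction and a switchable zero-gravity movement state.
; ToggleGravity swaps between Walking and Flying modes along with capsule gravity, while movement axes push along the capsule's forward, right and up vectors.
; Every tick, a short camera line trace caches the hit Interactable if it can be interacted with, otherwise clears it.
; The Interact input begins interaction on that cached target.
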(event `InputAction|Jump`
  (params (Key :type "Key Structure"))
  ;[1 1 1] Action Mapping
  (:`Pressed`
    (`self.Jump`)))

(event `InputAxis|Turn Right / Left Mouse`
  (params (AxisValue :type "Float (single-precision)"))
  ;[1 1 1] Camera
  (`self.AddControllerYawInput` AxisValue))

(event `InputAxis|Look Up / Down Mouse`
  (params (AxisValue :type "Float (single-precision)"))
  ;[1 1 1] Camera
  (`self.AddControllerPitchInput` AxisValue))

(event `/Game/HaileyStuff/Blueprints/IF_Gravity.ToggleGravity`
  (params (hasGravity :type Boolean))
  ;[1 1 1] Zero Gravity
  (if hasGravity
    (`CharacterMovementComponent.SetMovementMode` (`self.CharacterMovement`) "MOVE_Walking" 0)
    (`PrimitiveComponent.SetEnableGravity` (`self.CapsuleComponent`) true)
    (else
      (`CharacterMovementComponent.SetMovementMode` (`self.CharacterMovement`) "MOVE_Flying" 0)
      (`PrimitiveComponent.SetEnableGravity` (`self.CapsuleComponent`) false))))

(event `InputAxis|Move Forward / Backward`
  (params (AxisValue :type "Float (single-precision)"))
  ;[1 1 1] Movement
  (`self.AddMovementInput` (`SceneComponent.GetForwardVector` (`self.CapsuleComponent`)) AxisValue))

(event `InputAxis|Move Right / Left`
  (params (AxisValue :type "Float (single-precision)"))
  ;[1 1 1] Movement
  (`self.AddMovementInput` (`SceneComponent.GetRightVector` (`self.CapsuleComponent`)) AxisValue))

(event `InputAction|Interact`
  (params (Key :type "Key Structure"))
  (bind _currentinteractable (`self.CurrentInteractable`))
  ;[1 1 1] Interact
  (:`Pressed`
    (`/Engine/EditorBlueprintResources/StandardMacros.IsValid` _currentinteractable
      (:`Is Valid`
        (`/Game/HaileyStuff/Blueprints/Interactable.BeginInteraction` _currentinteractable)))))

(event `InputAxis|Move Up / Down`
  (params (AxisValue :type "Float (single-precision)"))
  ;[1 1 1] Movement
  (`self.AddMovementInput` (`SceneComponent.GetUpVector` (`self.CapsuleComponent`)) AxisValue))

(event `self.ReceiveTick`
  (params (DeltaSeconds :type "Float (single-precision)"))
  (bind _camera (`self.Camera`))
  (bind _returnvalue (`SceneComponent.K2_GetComponentLocation` _camera))
  ;[1 1 1] Event TIck
  (bind _outhit (`KismetSystemLibrary.LineTraceSingle` _returnvalue (+ _returnvalue (* (`KismetMathLibrary.GetForwardVector` (`SceneComponent.K2_GetComponentRotation` _camera)) 250.0)) "TraceTypeQuery1"))
  (bind _asinteractable (cast `/Game/HaileyStuff/Blueprints/Interactable` (`.HitActor` (`GameplayStatics.BreakHitResult` _outhit)))
    (:`then`
      (if (`/Game/HaileyStuff/Blueprints/Interactable.CanInteract` _asinteractable)
        (set `self.CurrentInteractable` _asinteractable)
        (else
          (set `self.CurrentInteractable` null :!label _label))))
    (:`CastFailed`
      (goto _label))))

(fn `UserConstructionScript`)