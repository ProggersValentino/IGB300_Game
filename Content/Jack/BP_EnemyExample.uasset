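; BP_EnemyExample is an example enemy Blueprint that tracks the gladiator player and exposes simple state queries.
; BeginPlay caches the first BP_WWEGladiator_Player found, and Tick copies that actor's location into TargetMovePos every frame.
; Helper functions report the Stunned and Fearing flags and whether the enemy is within a distance limit of that target.
; The file itself contains no movement logic and never sets either flag.
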(event `self.ReceiveBeginPlay`
  (bind _returnvalue (`GameplayStatics.GetActorOfClass` "/Game/BluePrints/Player/GladiatorRelated/BP_WWEGladiator_Player.BP_WWEGladiator_Player_C"))
  (set `self.PlayerReference` _returnvalue))

(event `self.ReceiveTick`
  (params (DeltaSeconds :type "Float (single-precision)"))
  (set `self.TargetMovePos` (`self.K2_GetActorLocation` (`self.PlayerReference`))))

(fn `isCloseToTarget`
  (returns (Close :type Boolean))
  (return (< (`KismetMathLibrary.Vector_Distance` (`self.K2_GetActorLocation`) (`self.TargetMovePos`)) (`self.IsCloseToTargetLimit`))))

(fn `isFearing`
  (returns (Fearing :type Boolean))
  (return (`self.Fearing`)))

(fn `isStunned`
  (returns (Stunned :type Boolean))
  (return (`self.Stunned`)))

(fn `UserConstructionScript`)