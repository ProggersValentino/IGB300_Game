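; Spawner actor that throws an interactable ball along a spline and turns it into a random item when it lands in its overlap.
; BeginPlay spawns a physics-enabled ball at a random ThrowLocation and tracks it in FlyingActors.
; Tick pushes tracked balls with impulses along the nearest spline tangent, stopping at the spline's end.
; An overlapping ball is replaced by a random class from Items at its location.
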(event `self.ReceiveBeginPlay`
  (`self.SpawnThrownItem`))

(event `self.ReceiveActorBeginOverlap`
  (params (OtherActor :type "Actor Object Reference"))
  (bind _asinteractable_ball (cast `/Game/BluePrints/InteractableSystem/Items/Interactable_Ball` OtherActor))
  (bind _output_get (set `self.Thrown Item` _asinteractable_ball))
  (bind _item (`self.DetermineItem`))
  (`self.SpawnItem` _item (`SceneComponent.K2_GetComponentLocation` (`/Game/BluePrints/InteractableSystem/Items/Interactable_Ball.Ball` _output_get)))
  (`KismetSystemLibrary.DelayUntilNextTick`)
  (`self.K2_DestroyActor` (`self.Thrown Item`)))

(event `self.ReceiveTick`
  (params (DeltaSeconds :type "Float (single-precision)"))
  (for (_array_element _array_index) (`self.FlyingActors`)
    (`/Engine/EditorBlueprintResources/StandardMacros.IsValid` _array_element
      (:`Is Valid`
        (`self.ApplySplinePhysics` (`/Game/BluePrints/InteractableSystem/Items/Interactable_Ball.Ball` _array_element) DeltaSeconds (`|GetArrayItem` (`self.Indices`) _array_index))))))

(fn `AddPhysics`
  (params (Primitive :type "PrimitiveComponent Object Reference"))
  (`PrimitiveComponent.SetCollisionEnabled` Primitive "NoCollision")
  (`PrimitiveComponent.SetSimulatePhysics` Primitive true)
  (`PrimitiveComponent.SetCollisionEnabled` Primitive "QueryAndPhysics")
  (`PrimitiveComponent.SetEnableGravity` Primitive true))

(fn `ApplySplinePhysics`
  (params (FlyingActor :type "PrimitiveComponent Object Reference") (DeltaSecs :type "Float (double-precision)") (ThrowIndex :type Integer))
  (locals (Distance :type "Float (single-precision)" :default 0.0) (Time :type "Float (single-precision)" :default 0.0))
  (bind _flyingactors (`self.FlyingActors`))
  (bind _spline (`/Game/BluePrints/InteractableSystem/BP_ItemLocation.Spline` (`|GetArrayItem` (`self.throwLocation`) ThrowIndex)))
  (bind _output_get (set `local.Distance` (`SplineComponent.GetDistanceAlongSplineAtLocation` _spline (`SceneComponent.K2_GetComponentLocation` FlyingActor) "World")))
  (bind _returnvalue (`SplineComponent.GetLocationAtDistanceAlongSpline` _spline _output_get "World"))
  (`KismetSystemLibrary.DrawDebugArrow` _returnvalue (+ (`SplineComponent.GetTangentAtDistanceAlongSpline` _spline _output_get "World") _returnvalue) 5.0 (`KismetMathLibrary.LinearColorLerp` (struct :`R` 1.0 :`G` 1.0 :`B` 1.0 :`A` 1.0) (struct :`R` 1.0 :`A` 1.0) (`local.Time`)))
  (set `local.Time` (`SplineComponent.GetTimeAtDistanceAlongSpline` _spline _output_get))
  (`PrimitiveComponent.AddImpulse` (`local.FlyingActor`) (* (`local.DeltaSecs`) (`SplineComponent.GetTangentAtDistanceAlongSpline` _spline (`local.Distance`) "World") (`self.Acceleration`)) "None" false)
  (if (>= (`local.Time`) 1.0)
    (`KismetArrayLibrary.Array_RemoveItem` _flyingactors)
    (if (== (`KismetArrayLibrary.Array_Length` _flyingactors) 0)
      (`self.SetActorTickEnabled` false))))

(fn `DetermineItem`
  (returns (Item :type "/Game/BluePrints/InteractableSystem/Interactable Class Reference"))
  (return (`KismetArrayLibrary.Array_Random` (`self.Items`))))

(fn `SpawnItem`
  (params (Item :type "/Game/BluePrints/InteractableSystem/Interactable Class Reference") (Location :type "Vector Structure"))
  (`|SpawnActorFromClass` Item (`KismetMathLibrary.MakeTransform` Location) "AlwaysSpawn" "MultiplyWithRoot" null null)
  (`KismetSystemLibrary.PrintString` "spawned!!"))

(fn `SpawnThrownItem`
  (bind (_outitem _outindex) (`KismetArrayLibrary.Array_Random` (`self.throwLocation`)))
  (bind _returnvalue (`|SpawnActorFromClass` "/Game/BluePrints/InteractableSystem/Items/Interactable_Ball.Interactable_Ball_C" (`self.GetTransform` _outitem) "Undefined" "MultiplyWithRoot" null null))
  (`self.AddPhysics` (`/Game/BluePrints/InteractableSystem/Items/Interactable_Ball.Ball` _returnvalue))
  (`self.AddPhysics` (`/Game/BluePrints/InteractableSystem/Interactable.Niagara` _returnvalue))
  (`KismetArrayLibrary.Array_Add` (`self.FlyingActors`) _returnvalue)
  (`KismetArrayLibrary.Array_Add` (`self.Indices`) _outindex)
  (`self.SetActorTickEnabled` true))

(fn `UserConstructionScript`)