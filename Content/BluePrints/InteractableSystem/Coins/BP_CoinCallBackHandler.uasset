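; Coin pickup handler actor that spawns Niagara coin particles and credits the player when they are absorbed.
; SpawnCoins launches coin systems, and Tick feeds each the player's offset mesh position as PlayerPos.
; The Niagara ParticleData callback applies the coin GameplayEffect for particles within pickup range, updating the coin widget and crowd subsystem's Aureus.
; Each pickup plays a sound with rising, clamped pitch that resets after a retriggerable delay.
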(event `self.ReceiveBeginPlay`
  (bind _coinsniagara (`self.CoinsNiagara`))
  (`KismetSystemLibrary.K2_SetTimer` null "Spawn" 5.0)
  (`NiagaraComponent.SetVariableObject` _coinsniagara "BPCallBackHandler" self)
  (`KismetArrayLibrary.Array_AddUnique` (`self.NiagraObjectArray`) _coinsniagara))

(event `SpawnCoins`
  (params (NumberOfCoins :type "Float (double-precision)"))
  (bind _coinsniagara (`self.CoinsNiagara`))
  (`FXSystemComponent.SetFloatParameter` _coinsniagara "SpawnRate" NumberOfCoins)
  (`ActorComponent.Activate` _coinsniagara false)
  (bind _returnvalue (`NiagaraFunctionLibrary.SpawnSystemAttached` (`NiagaraComponent.GetAsset` _coinsniagara) _coinsniagara "None" (0.0 0.0 0.0) (struct) "KeepRelativeOffset"))
  (`KismetArrayLibrary.Array_AddUnique` (`self.NiagraObjectArray`) _returnvalue))

(event `self.ReceiveTick`
  (params (DeltaSeconds :type "Float (single-precision)"))
  (bind _returnvalue (`GameplayStatics.GetPlayerCharacter` 0))
  (if (`KismetSystemLibrary.IsValid` _returnvalue)
    (for _array_element (`self.NiagraObjectArray`)
      (`NiagaraComponent.SetVariablePosition` _array_element "PlayerPos" (+ (`SceneComponent.K2_GetComponentLocation` (`Character.Mesh` _returnvalue)) (`self.PlayerAbsorbOffset`))))))

(event `self.MS_Coins.OnAudioFinished`
  (set `self.IsFinished` true))

(event `self.ReceiveParticleData`
  (params (Data :type "Array of BasicParticleData Structure (by ref)") (NiagaraSystem :type "NiagaraSystem Object Reference") (SimulationPositionOffset :type "Vector Structure (by ref)"))
  (bind _returnvalue (`GameplayStatics.GetPlayerCharacter` 0))
  (bind _basecoinamount (`self.BaseCoinAmount`))
  (bind _ms_coins (`self.MS_Coins`))
  (for _array_element Data
    (if (< (`KismetMathLibrary.Vector_Distance` (+ (`SceneComponent.K2_GetComponentLocation` (`Character.Mesh` (`GameplayStatics.GetPlayerCharacter` 0))) (`self.PlayerAbsorbOffset`)) (break `BasicParticleData` _array_element)) (`self.PickUpCheckRange`))
      (if (`KismetSystemLibrary.IsValid` _returnvalue)
        (`AbilitySystemComponent.BP_ApplyGameplayEffectToSelf` :`self` (`AbilitySystemBlueprintLibrary.GetAbilitySystemComponent` _returnvalue) :`GameplayEffectClass` "/Game/BluePrints/InteractableSystem/GameEffects/GE_Item_Coin.GE_Item_Coin_C" :`Level` 1.0)
        (`/Game/BluePrints/UI/Widgets/WBP_CoinUI.SpawnUICoins` (`self.CoinWidget`))
        (`/Game/BluePrints/UI/Widgets/WBP_CoinUI.AddToBonus` (`self.CoinWidget`) _basecoinamount)
        (`CrowdWorldSubsystem.UpdateAureus` (subsystem `CrowdWorldSubsystem`) _basecoinamount)
        (if true
          (bind _output_get (set `self.CurrentPitch` (`KismetMathLibrary.FClamp` (+ (`self.CurrentPitch`) 0.2) -2.0 2.0)))
          (`AudioComponent.SetPitchMultiplier` _ms_coins _output_get)
          (`AudioComponent.Play` _ms_coins 0.0)
          (`KismetSystemLibrary.RetriggerableDelay` 2.0)
          (set `self.CurrentPitch` -2.0))))))

(fn `UserConstructionScript`)