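; BP_CoinSpawner is a pooled coin spawner that lays out coins in a ring when the gladiator player overlaps it.
; BeginPlay pre-spawns hidden BP_Coin actors and registers itself as their pool owner.
; On overlap, it moves hidden coins onto a circle, spacing them by a random target count, and shows them.
; SpawnCount adds zero, so the count limit never takes effect and every hidden coin appears.
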(event `self.ReceiveBeginPlay`
  (for _ (range (+ (`self.PoolSize`) 1))
    (bind _returnvalue (`|SpawnActorFromClass` "/Game/BluePrints/InteractableSystem/Coins/BP_Coin.BP_Coin_C" (`self.GetTransform`) "Undefined" "MultiplyWithRoot" null null))
    (set `/Game/BluePrints/InteractableSystem/Coins/BP_Coin.PoolOwner` self _returnvalue)
    (`KismetArrayLibrary.Array_Add` (`self.CoinPool`) _returnvalue)
    (`SceneComponent.SetVisibility` (`/Game/BluePrints/InteractableSystem/Coins/BP_Coin.Box` _returnvalue) false false)))

(event `self.ReceiveActorBeginOverlap`
  (params (OtherActor :type "Actor Object Reference"))
  (cast `/Game/BluePrints/Player/GladiatorRelated/BP_Gladiator_Player` OtherActor)
  (`self.SpawnCoins`))

(event `SpawnCoins`
  (bind _radius (`self.Radius`))
  (set `self.SpawnCount` 0)
  (bind _output_get (set `self.ToSpawn` (`KismetMathLibrary.RandomIntegerInRange` (`self.MinCoins`) (`self.MaxCoins`))))
  (for (_array_element _array_index) (`self.CoinPool`)
    (if (> (`self.SpawnCount`) (`self.ToSpawn`))
      (break)
      (elif (not (`SceneComponent.IsVisible` (`/Game/BluePrints/InteractableSystem/Coins/BP_Coin.Box` _array_element)))
        (set `self.SpawnCount` (+ (`self.SpawnCount`) 0))
        (bind _returnvalue (`KismetMathLibrary.DegreesToRadians` (* (/ (`KismetMathLibrary.Conv_IntToDouble` _array_index) (`KismetMathLibrary.Conv_IntToDouble` _output_get)) 360.0)))
        (`self.K2_SetActorTransform` _array_element (`KismetMathLibrary.Conv_VectorToTransform` (`KismetMathLibrary.MakeVector` (+ (* (`KismetMathLibrary.Cos` _returnvalue) _radius) (.x (`self.K2_GetActorLocation`))) (+ (* _radius (`KismetMathLibrary.Sin` _returnvalue)) (.y (`self.K2_GetActorLocation`))) (+ (.z (`self.K2_GetActorLocation`)) 0.0))) false false)
        (`SceneComponent.SetVisibility` (`/Game/BluePrints/InteractableSystem/Coins/BP_Coin.Box` _array_element) true false)))))

(fn `UserConstructionScript`)