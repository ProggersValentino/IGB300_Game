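; Gameplay ability that knocks back a gladiator when the player triggers it through a gameplay event.
; It applies GE_KnockBack to the event's target data using the event's context.
; It then launches the target along the instigating player's follow-camera forward and up vectors, adding to existing velocity, so aim sets the direction.
; The ability ends only after the launch, so a failed instigator or target cast leaves it active.
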(event `self.K2_ActivateAbilityFromEvent`
  (params (EventData :type "GameplayEventData Structure (by ref)"))
  (bind (_eventtag _instigator _target _optionalobject _optionalobject2 _contexthandle _instigatortags _targettags _eventmagnitude _targetdata) (break `GameplayEventData` EventData))
  (`self.K2_ApplyGameplayEffectSpecToTarget` (`AbilitySystemComponent.MakeOutgoingSpec` (`AbilitySystemBlueprintLibrary.GetAbilitySystemComponent` (`self.GetOwningActorFromActorInfo`)) "/Game/BluePrints/Player/GladiatorRelated/Abilities/KnockBack/GE_KnockBack.GE_KnockBack_C" 1.0 _contexthandle) _targetdata)
  (bind _asbp_wwegladiator_player (cast `/Game/BluePrints/Player/GladiatorRelated/BP_WWEGladiator_Player` _instigator))
  (bind _asgladiator_base_char (cast `GladiatorBaseChar` _target))
  (bind _followcamera (`/Game/BluePrints/Player/GladiatorRelated/BP_WWEGladiator_Player.FollowCamera` _asbp_wwegladiator_player))
  (`Character.LaunchCharacter` _asgladiator_base_char (+ (* (`SceneComponent.GetForwardVector` _followcamera) 2500.0) (* (`SceneComponent.GetUpVector` _followcamera) 1000.0)) false false)
  (`self.K2_EndAbility`))