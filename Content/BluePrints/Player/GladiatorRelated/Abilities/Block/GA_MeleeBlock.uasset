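; Gameplay ability for the Gladiator's melee block, which holds GE_Block while playing a block montage.
; Effects applied from sources tagged with a forward hit direction trigger recoil and brace cues on attacker and blocker, and grant GE_BlockedRage.
; Event.Block.End plays an exit montage, then ends the ability, which removes the last stored block effect handle.
; Montage interruption cancels the running tasks and waits for Event.Montage.Block to restart the block.
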(event `self.K2_ActivateAbility`
  (bind _returnvalue (`self.K2_CommitAbility`))
  (if _returnvalue
    (bind _asynctaskproxy (`AbilityTask_PlayMontageAndWait.CreatePlayMontageAndWaitProxy` "None" "/Game/BluePrints/Player/GladiatorRelated/Anim/Montages/AM_WWE_Gladiator_Block.AM_WWE_Gladiator_Block" :!label _label)
      (:`then`
        (set `self.Async_MontageTask` _asynctaskproxy)
        (`|ExecutionSequence`
          (:`then_0`
            (bind _returnvalue_2 (`self.BP_ApplyGameplayEffectToOwner` "/Game/BluePrints/Player/GladiatorRelated/Abilities/Block/GE_Block.GE_Block_C"))
            (set `self.BlockHandle` _returnvalue_2) ; allow us to remove the ability when we end the block
          )
          (:`then_1`
            (bind _asynctaskproxy_2 (`AbilityTask_WaitGameplayEvent.WaitGameplayEvent` (struct :`TagName` "Event.Block.End") null true)
              (:`then`
                (set `self.Async_BlockEnd` _asynctaskproxy_2))
              (:`EventReceived`
                (`self.EndBlock`))))
          (:`then_2`
            (bind (_asynctaskproxy_3 _source _spechandle) (`AbilityTask_WaitGameplayEffectApplied_Self.WaitGameplayEffectAppliedToSelf` (struct) (make `GameplayTagRequirements` (struct :`GameplayTags` (struct :`(TagName` "Gameplay.HitDirection.Forward")))) (struct) false null)
              (:`then`
                (set `self.Async_GettingAttacked` _asynctaskproxy_3))
              (:`OnApplied`
                (bind _returnvalue_3 (`AbilitySystemBlueprintLibrary.GetEffectContext` _spechandle))
                ;[1 1 1] block recoil reaction + block brace reaction gameplay cues
                (`GameplayCueFunctionLibrary.ExecuteGameplayCueOnActor` _source (struct :`TagName` "GameplayCue.HitReact.Block") (`AbilitySystemBlueprintLibrary.MakeGameplayCueParameters` 0.0 0.0 _returnvalue_3))
                (`GameplayCueFunctionLibrary.ExecuteGameplayCueOnActor` (`self.GetAvatarActorFromActorInfo`) (struct :`TagName` "GameplayCue.HitReact.BraceBlock") (`AbilitySystemBlueprintLibrary.MakeGameplayCueParameters` 0.0 0.0 _returnvalue_3))
                (`self.BP_ApplyGameplayEffectToOwner` "/Game/BluePrints/Player/GladiatorRelated/Abilities/Block/BlockedRage/GE_BlockedRage.GE_BlockedRage_C"))))))
      (:`OnInterrupted`
        (`AbilityTask_WaitGameplayEvent.WaitGameplayEvent` (struct :`TagName` "Event.Montage.Block") null true ; On interrupted, wait for call to reset animation while ability active
          (:`then`
            (`self.AbortTasksEarly`))
          (:`EventReceived`
            (goto _label)))))
    (else
      (`self.K2_EndAbility`))))

(event `self.K2_OnEndAbility`
  (params (bWasCancelled :type Boolean))
  (`self.BP_RemoveGameplayEffectFromOwnerWithHandle` (`self.BlockHandle`)))

(event `EndBlock`
  (`AbilityTask_PlayMontageAndWait.CreatePlayMontageAndWaitProxy` "None" "/Game/ArtAssets/Animation/Animation/PC_AnimNOSWORD/AM_Gladiator_BlockNoSword.AM_Gladiator_BlockNoSword" 1.0 "EndBlock"
    (:`OnCompleted`
      _)
    (:`OnBlendOut`
      _)
    (:`OnInterrupted`
      _))
  (`self.K2_EndAbility`))

(event `AbortTasksEarly`
  (`GameplayTask.EndTask` (`self.Async_GettingAttacked`))
  (`GameplayTask.EndTask` (`self.Async_BlockEnd`))
  (`GameplayTask.EndTask` (`self.Async_MontageTask`)))