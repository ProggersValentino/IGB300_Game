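; Gameplay ability that plays a gladiator's uppercut hit reaction, acting as a stun.
; On activation it disables character movement, prints a debug "stunned" message and plays the uppercut montage.
; Only montage completion ends the ability and restores walking; interruption and cancellation are not handled on the live path.
; An unconnected leftover branch holds a faster jumpscare reaction montage.
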(event `self.K2_ActivateAbility`
  (bind _asgladiator_base_char (cast `GladiatorBaseChar` (`self.GetAvatarActorFromActorInfo`)))
  (`CharacterMovementComponent.DisableMovement` (`Character.CharacterMovement` _asgladiator_base_char))
  (`KismetSystemLibrary.PrintString` "stunned" true true (struct :`R` 1.0 :`G` 0.988195 :`B` 0.583724 :`A` 1.0))
  (`AbilityTask_PlayMontageAndWait.CreatePlayMontageAndWaitProxy` "None" "/Game/BluePrints/Player/GladiatorRelated/Anim/Montages/AM_WWEGladiator_HitReaction_UpperCut.AM_WWEGladiator_HitReaction_UpperCut"
    (:`OnCompleted`
      (`self.K2_EndAbility`)
      (`CharacterMovementComponent.SetMovementMode` (`Character.CharacterMovement` _asgladiator_base_char) "MOVE_Walking" 0))))