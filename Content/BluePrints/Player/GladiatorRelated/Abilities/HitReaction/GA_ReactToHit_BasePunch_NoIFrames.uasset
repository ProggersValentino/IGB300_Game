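; Gameplay ability for a gladiator's hit reaction to a base punch, with no invincibility frames applied.
; On activation it disables character movement, fires the BasePunch gameplay cue and plays the spin hit-reaction montage.
; Only montage completion ends the ability and restores walking; interruption and cancellation are unhandled on the live path, and an alternate Jumpscare montage branch sits unconnected.
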(event `self.K2_ActivateAbility`
  (bind _asgladiator_base_char (cast `GladiatorBaseChar` (`self.GetAvatarActorFromActorInfo`)))
  (`CharacterMovementComponent.DisableMovement` (`Character.CharacterMovement` _asgladiator_base_char))
  (`GameplayCueFunctionLibrary.ExecuteGameplayCueOnActor` (`self.GetAvatarActorFromActorInfo`) (struct :`TagName` "GameplayCue.Ability.BasePunch") (`AbilitySystemBlueprintLibrary.MakeGameplayCueParameters` 0.0))
  (`AbilityTask_PlayMontageAndWait.CreatePlayMontageAndWaitProxy` "None" "/Game/BluePrints/Player/GladiatorRelated/Anim/Montages/AM_WWEGladiator_HitReaction_Spin.AM_WWEGladiator_HitReaction_Spin"
    (:`OnCompleted`
      (`self.K2_EndAbility`)
      (`CharacterMovementComponent.SetMovementMode` (`Character.CharacterMovement` _asgladiator_base_char) "MOVE_Walking" 0))))