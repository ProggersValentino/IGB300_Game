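; Gameplay ability that plays the gladiator's hit reaction while granting temporary invincibility frames.
; On activation it disables character movement, starts the jumpscare hit-reaction montage sped up, and applies the temporary i-frames effect to the owner.
; After a short delay it replays the montage from its "end" section at default rate.
; That montage finishing, or either being interrupted or cancelled, ends the ability and restores walking.
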(event `self.K2_ActivateAbility`
  (bind _asgladiator_base_char (cast `GladiatorBaseChar` (`self.GetAvatarActorFromActorInfo`)))
  (`CharacterMovementComponent.DisableMovement` (`Character.CharacterMovement` _asgladiator_base_char))
  (`AbilityTask_PlayMontageAndWait.CreatePlayMontageAndWaitProxy` "None" "/Game/BluePrints/Player/GladiatorRelated/Anim/Montages/AM_WWEGladiator_HitReaction_Jumpscare.AM_WWEGladiator_HitReaction_Jumpscare" 3.0
    (:`then`
      (`self.K2_ApplyGameplayEffectSpecToOwner` (`self.MakeOutgoingGameplayEffectSpec` "/Game/BluePrints/Player/GladiatorRelated/Abilities/GE_IFrames_Temporary.GE_IFrames_Temporary_C"))
      (`KismetSystemLibrary.Delay` 0.23)
      (`AbilityTask_PlayMontageAndWait.CreatePlayMontageAndWaitProxy` "None" "/Game/BluePrints/Player/GladiatorRelated/Anim/Montages/AM_WWEGladiator_HitReaction_Jumpscare.AM_WWEGladiator_HitReaction_Jumpscare" 1.0 "end"
        (:`OnCompleted`
          _)
        (:`OnInterrupted`
          _)
        (:`OnCancelled`
          _))
      (`self.K2_EndAbility`)
      (`CharacterMovementComponent.SetMovementMode` (`Character.CharacterMovement` _asgladiator_base_char) "MOVE_Walking" 0))
    (:`OnInterrupted`
      (`self.K2_EndAbility` :!label _label)
      (`CharacterMovementComponent.SetMovementMode` (`Character.CharacterMovement` _asgladiator_base_char) "MOVE_Walking" 0))
    (:`OnCancelled`
      (goto _label))))