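; Gameplay ability for the WWE Gladiator player's right base punch melee attack.
; After committing, it plays the punch montage and waits for the montage's gameplay event.
; On that event, it applies GE_ShortSlash to the payload's targets with stat-adjusted SetByCaller damage and fires the punch gameplay cue.
; Montage exit restores walking, then tries the next attack type on completion or blend-out, or engages input queuing on interruption or cancellation.
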(event `self.K2_ActivateAbility`
  (bind _returnvalue (`self.K2_CommitAbility`))
  (if _returnvalue
    (bind _asbp_wwegladiator_player (cast `/Game/BluePrints/Player/GladiatorRelated/BP_WWEGladiator_Player` (`self.GetAvatarActorFromActorInfo`)))
    (`AbilityTask_PlayMontageAndWait.CreatePlayMontageAndWaitProxy` "None" "/Game/BluePrints/Player/GladiatorRelated/Anim/Montages/AM_WWE_Gladiator_BasePunch.AM_WWE_Gladiator_BasePunch"
      (:`then`
        (bind (_asynctaskproxy _payload) (`AbilityTask_WaitGameplayEvent.WaitGameplayEvent` (struct :`TagName` "Event.Montage.BasePunch") null)
          (:`EventReceived`
            (bind (_eventtag _instigator _target _optionalobject _optionalobject2 _contexthandle _instigatortags _targettags _eventmagnitude _targetdata) (break `GameplayEventData` _payload))
            (bind _returnvalue_2 (`GladiatorEffectContextLibrary.GetStatAdjustment` _optionalobject))
            (bind _returnvalue_3 (`AbilitySystemBlueprintLibrary.AssignSetByCallerMagnitude` (`AbilitySystemComponent.MakeOutgoingSpec` (`AbilitySystemBlueprintLibrary.GetAbilitySystemComponent` (`self.GetOwningActorFromActorInfo`)) "/Game/BluePrints/Player/GladiatorRelated/Abilities/Melee/GE_ShortSlash.GE_ShortSlash_C" 0.0 _contexthandle) "AddDmg" (`StatAdjustment.damageAdjustment` _returnvalue_2)))
            (`self.K2_ApplyGameplayEffectSpecToTarget` _returnvalue_3 _targetdata)
            (`GameplayCueFunctionLibrary.ExecuteGameplayCueOnActor` _target (struct :`TagName` "GameplayCue.Ability.BasePunch") (`AbilitySystemBlueprintLibrary.MakeGameplayCueParameters` 0.0 0.0 _contexthandle (struct) (struct) (struct) (struct) (0.0 0.0 0.0) (0.0 0.0 0.0) _instigator)))))
      (:`OnCompleted`
        (`self.K2_EndAbility` :!label _label)
        (bind _charactermovement (`Character.CharacterMovement` _asbp_wwegladiator_player))
        (`CharacterMovementComponent.SetMovementMode` _charactermovement "MOVE_Walking" 0)
        (`GladiatorPlayerChar.TryActivateAttackType` _asbp_wwegladiator_player))
      (:`OnBlendOut`
        (goto _label))
      (:`OnInterrupted`
        (`self.K2_EndAbility` :!label _label_2)
        (`CharacterMovementComponent.SetMovementMode` _charactermovement "MOVE_Walking" 0)
        (`GladiatorPlayerChar.EngageInputQueuing` _asbp_wwegladiator_player))
      (:`OnCancelled`
        (goto _label_2)))
    (else
      (`self.K2_EndAbility`))))