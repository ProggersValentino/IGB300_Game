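; BP_Maestro directs the gladiator arena game loop, running waves and rounds until a win screen after five rounds.
; NextRound sets difficulty by round and spawns enemies through EnemySubsystem, while Tick polls only for melee enemies to advance waves.
; Round end plays a random sequence, shows the end screen, grows the crowd and adds a wave.
; It also creates shared screen-wipe and loading widgets and awards achievements after round five.
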(event `TauntTut`
  (`self.TauntTutorial`))

(event `self.ReceiveTick`
  (params (DeltaSeconds :type "Float (single-precision)"))
  (bind _outactors (`GameplayStatics.GetAllActorsOfClass` "/Game/BluePrints/AI/EnemyRelated/Enemies/BP_BasicMeleeEnemy.BP_BasicMeleeEnemy_C"))
  (if (and (<= (`KismetArrayLibrary.Array_Length` _outactors) 0) (== (`self.State`) "Round"))
    (bind _output_get (set `self.CurrentWave` (+ (`self.CurrentWave`) 1)))
    (if (>= _output_get (`self.NumWaves`))
      (set `self.NumWaves` (+ (`self.NumWaves`) 1))
      (set `self.CurrentWave` 0)
      (`self.BeginEndOfRound`)
      (`self.SetActorTickEnabled` false)
      (else
        (if (== (`self.RoundCounter`) 0)
          (set `self.Difficulty` "NORMAL"))
        (`EnemySubsystem.TrySpawn` (subsystem `EnemySubsystem`) (`self.Difficulty`) "/Game/BluePrints/AI/EnemyRelated/Enemies/BP_BasicMeleeEnemy.BP_BasicMeleeEnemy_C")))))

(event `self.ReceiveBeginPlay`
  (bind _player (`self.Player`))
  (bind _asbp_wwegladiator_player (cast `/Game/BluePrints/Player/GladiatorRelated/BP_WWEGladiator_Player` (`GameplayStatics.GetPlayerCharacter` 0)))
  (set `self.Player` _asbp_wwegladiator_player)
  (bind _returnvalue (`|CreateWidget` "/Game/BluePrints/UI/WP_LoadingScreen.WP_LoadingScreen_C"))
  (bind _output_get (set `self.LoadingScreen` _returnvalue))
  (`Widget.SetVisibility` _output_get "Hidden")
  (`UserWidget.AddToViewport` _output_get 0)
  (bind _returnvalue_2 (`|CreateWidget` "/Game/BluePrints/UI/WP_ScreenWipe.WP_ScreenWipe_C" (`GameplayStatics.GetPlayerController` 0)))
  (bind _output_get_2 (set `self.ScreenWipe` _returnvalue_2))
  (`UserWidget.AddToViewport` _output_get_2 0)
  (set `/Game/BluePrints/Player/GladiatorRelated/BP_WWEGladiator_Player.Screen Wipe` _output_get_2 _player)
  (set `/Game/BluePrints/Player/GladiatorRelated/BP_WWEGladiator_Player.LoadingScreen` (`self.LoadingScreen`) _player)
  (`self.NextRound`))

(event `BeginEndOfRound`
  (bind _returnvalue (`GameplayStatics.GetPlayerController` 0))
  (bind _returnvalue_2 (`GameplayStatics.GetPlayerController` 0))
  (bind _returnvalue_3 (`GameplayStatics.GetPlayerController` 0))
  (bind _returnvalue_4 (subsystem `CrowdWorldSubsystem`))
  (bind _returnvalue_5 (+ (`CrowdWorldSubsystem.GetCrowdSize` _returnvalue_4) 1000))
  (set `self.State` "EndRound")
  (`KismetSystemLibrary.Delay` 1.0)
  (`self.StartSequence` (`KismetArrayLibrary.Array_Random` (`self.EndRoundSequences`)))
  (set `self.RoundCounter` (+ (`self.RoundCounter`) 1))
  (bind _returnvalue_6 (`|CreateWidget` "/Game/BluePrints/UI/EndScreen/WB_EndScreen.WB_EndScreen_C" (`GameplayStatics.GetPlayerController` 0)))
  (bind _output_get (set `self.endOfRoundWidget` _returnvalue_6))
  (`UserWidget.AddToViewport` _output_get 0)
  (set `/Game/BluePrints/UI/EndScreen/WB_EndScreen.ScreenWipe` (`self.ScreenWipe`) _returnvalue_6)
  (set `/Game/BluePrints/UI/EndScreen/WB_EndScreen.LoadingScreen` (`self.LoadingScreen`) _returnvalue_6)
  (`CrowdWorldSubsystem.SetCrowdSize` _returnvalue_4 _returnvalue_5)
  (bind _returnvalue_7 (`GameplayStatics.GetActorOfClass` "/Game/BluePrints/GlorySystem/CrowdVFX/BP_VFXCrowdController.BP_VFXCrowdController_C"))
  ;[1 1 1] Reward Champion
  (set `/Game/BluePrints/GlorySystem/CrowdVFX/BP_VFXCrowdController.CurrentCrowdSize` (`KismetMathLibrary.Conv_IntToDouble` _returnvalue_5) _returnvalue_7)
  (if (== (`self.RoundCounter`) 5)
    (`AchievementQueryCallbackProxy.CacheAchievements` _returnvalue_3
      (:`then`
        ;[1 1 1] Reward Bloodbath
        (if (>= (`GameplayStats.GetBloodSpilled` (subsystem `GameplayStats`)) 1000.0)
          (`AchievementQueryCallbackProxy.CacheAchievements` _returnvalue_2
            (:`OnSuccess`
              (bind (_bfoundid _progress) (`AchievementBlueprintLibrary.GetCachedAchievementProgress` _returnvalue_2 "BloodBath"))
              (if (not (== _progress 1.0))
                (`AchievementWriteCallbackProxy.WriteAchievementProgress` _returnvalue_2 "BloodBath" 1.0))))
          (else
            ;[1 1 1] Reward CrowdWeezer
            (if (<= (`CrowdWorldSubsystem.GetCumulativeExcitement` (subsystem `CrowdWorldSubsystem`)) 0.0)
              (`AchievementQueryCallbackProxy.CacheAchievements` _returnvalue
                (:`OnSuccess`
                  (bind (_bfoundid_2 _progress_2) (`AchievementBlueprintLibrary.GetCachedAchievementProgress` _returnvalue "CrowdWeezer"))
                  (if (not (== _progress_2 1.0))
                    (`AchievementWriteCallbackProxy.WriteAchievementProgress` _returnvalue "CrowdWeezer" 1.0))))))))
      (:`OnSuccess`
        (bind (_bfoundid_3 _progress_3) (`AchievementBlueprintLibrary.GetCachedAchievementProgress` _returnvalue_3 "Champion"))
        (if (not (== _progress_3 1.0))
          (`AchievementWriteCallbackProxy.WriteAchievementProgress` _returnvalue_3 "Champion" 1.0))))))

(event `StartSequence`
  (params (Sequence :type "LevelSequenceActor Object Reference"))
  (bind _sequenceplayer (`LevelSequenceActor.SequencePlayer` Sequence))
  (bind _player (`self.Player`))
  (`/Game/BluePrints/UI/WP_ScreenWipe.FadeOut` (`self.ScreenWipe`))
  (`/Engine/EditorBlueprintResources/StandardMacros.IsValid` Sequence
    (:`Is Valid`
      (`MovieSceneSequencePlayer.Play` _sequenceplayer)
      (`self.DisableInput` _player null)
      (`KismetSystemLibrary.Delay` (`TimeManagementBlueprintLibrary.Conv_QualifiedFrameTimeToSeconds` (`MovieSceneSequencePlayer.GetDuration` _sequenceplayer)))
      (`self.EnableInput` _player null))))

(event `NextRound`
  (bind _returnvalue (`GameplayStatics.GetPlayerController` 0))
  (bind (_returnvalue_x _returnvalue_y) (`KismetMathLibrary.BreakVector2D` (`WidgetLayoutLibrary.GetViewportSize`)))
  (`/Game/BluePrints/UI/WP_ScreenWipe.FadeOut` (`self.ScreenWipe`))
  (if (>= (`self.RoundCounter`) 5)
    (bind _returnvalue_2 (`|CreateWidget` "/Game/BluePrints/UI/Widgets/WBP_DeathUI.WBP_DeathUI_C" (`GameplayStatics.GetPlayerController` 0)))
    (set `TextBlock.Text` "You Won!" (`/Game/BluePrints/UI/Widgets/WBP_DeathUI.Lost_Base` _returnvalue_2))
    (set `TextBlock.Text` "You Won!" (`/Game/BluePrints/UI/Widgets/WBP_DeathUI.Lost_Shadow` _returnvalue_2))
    (`UserWidget.AddToViewport` _returnvalue_2 0)
    (`WidgetBlueprintLibrary.SetInputMode_GameAndUIEx` _returnvalue _returnvalue_2 "LockInFullscreen")
    (set `PlayerController.bShowMouseCursor` true _returnvalue)
    (`GameplayStatics.SetGamePaused` true)
    (`PlayerController.SetMouseLocation` _returnvalue (`KismetMathLibrary.FTrunc` (/ _returnvalue_x 2.0)) (`KismetMathLibrary.FTrunc` (/ _returnvalue_y 2.0)))
    (else
      (set `self.State` "Round")
      (if (== (`self.RoundCounter`) 2)
        (bind _output_get (set `self.Difficulty` "HARD"))
        (`EnemySubsystem.TrySpawn` (subsystem `EnemySubsystem`) _output_get "/Game/BluePrints/AI/EnemyRelated/Enemies/BP_BasicRangedEnemy.BP_BasicRangedEnemy_C")
        (`self.SetActorTickEnabled` true)
        (elif (== (`self.RoundCounter`) 4)
          (bind _output_get_2 (set `self.Difficulty` "HARDEST"))
          (`EnemySubsystem.TrySpawn` (subsystem `EnemySubsystem`) _output_get_2 "/Game/BluePrints/AI/EnemyRelated/Enemies/BP_BasicMeleeEnemy.BP_BasicMeleeEnemy_C")
          (`self.SetActorTickEnabled` true)
          (elif (== (`self.RoundCounter`) 0)
            (bind _output_get_3 (set `self.Difficulty` "EASY"))
            (`EnemySubsystem.TrySpawn` (subsystem `EnemySubsystem`) _output_get_3 "/Game/BluePrints/AI/EnemyRelated/Enemies/BP_BasicMeleeEnemy.BP_BasicMeleeEnemy_C")
            (`self.SetActorTickEnabled` true)
            (else
              (bind _output_get_4 (set `self.Difficulty` "NORMAL"))
              (`EnemySubsystem.TrySpawn` (subsystem `EnemySubsystem`) _output_get_4 "/Game/BluePrints/AI/EnemyRelated/Enemies/BP_BasicMeleeEnemy.BP_BasicMeleeEnemy_C")
              (`self.SetActorTickEnabled` true))))))))

(fn `UserConstructionScript`)