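; BP_EnemySpawnLightshow is an actor that plays a short light show with confetti and audio, presumably to mark enemy spawns.
; On BeginPlay it caches every BP_EnemySpotLight in the level and hides them along with its own component tree.
; BeginLightShow fires both confetti emitters and the audio, reveals the spotlights and components, then hides them again after a fixed delay.
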(event `self.ReceiveBeginPlay`
  (bind _outactors (`GameplayStatics.GetAllActorsOfClass` "/Game/BluePrints/BP_EnemySpotLight.BP_EnemySpotLight_C"))
  (bind _output_get (set `self.SpotLights` _outactors))
  (for _array_element _output_get
    (`self.SetActorHiddenInGame` _array_element true))
  (`SceneComponent.SetHiddenInGame` (`self.DefaultSceneRoot`) true true))

(event `BeginLightShow`
  (`ActorComponent.Activate` (`self.ConfettiLeft`) false)
  (`ActorComponent.Activate` (`self.ConfettiRight`) false)
  (`AudioComponent.Play` (`self.Audio`) 0.0)
  (for _array_element (`self.SpotLights`)
    (`self.SetActorHiddenInGame` _array_element false))
  (`SceneComponent.SetHiddenInGame` (`self.DefaultSceneRoot`) false true)
  (`KismetSystemLibrary.Delay` 5.0)
  (for _array_element_2 (`self.SpotLights`)
    (`self.SetActorHiddenInGame` _array_element_2 true))
  (`SceneComponent.SetHiddenInGame` (`self.DefaultSceneRoot`) true true))

(fn `UserConstructionScript`)