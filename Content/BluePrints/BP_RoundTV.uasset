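; BP_RoundTV is an in-world TV that displays the round number as part of a looping slideshow.
; ScrollImages calls itself every five seconds to swap the mesh material through TVMaterials.
; After each wrap, the WBP_TVSlideShow widget is shown alongside the first material and hidden for the others.
; SetRound updates the widget text, but its zero-round branch casts to WBP_ScorePopUpEffect instead and leaves Round unchanged.
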(event `self.ReceiveBeginPlay`
  (bind _aswbp_tvslide_show (cast `/Game/BluePrints/UI/Widgets/WBP_TVSlideShow` (`WidgetComponent.GetWidget` (`self.Widget`))))
  (set `self.TVSlide Show` _aswbp_tvslide_show)
  (set `TextBlock.Text` "1" (`/Game/BluePrints/UI/Widgets/WBP_TVSlideShow.TextBlock_139` _aswbp_tvslide_show))
  (`self.ScrollImages`))

(event `ScrollImages`
  (bind _index (`self.Index`))
  (bind _tvmaterials (`self.TVMaterials`))
  (`KismetSystemLibrary.Delay` 5.0)
  (`PrimitiveComponent.SetMaterial` (`self.StaticMeshComponent`) 0 (`|GetArrayItem` _tvmaterials _index))
  (bind _output_get (set `self.Index` (+ _index 1)))
  (`Widget.SetVisibility` (`self.TVSlide Show`) (`self.In Visibility`))
  (if (== _output_get (`KismetArrayLibrary.Array_Length` _tvmaterials))
    (set `self.Index` 0)
    (set `self.In Visibility` "Visible")
    (else
      (set `self.In Visibility` "Hidden")))
  (`self.ScrollImages`))

(fn `SetRound`
  (params (Round :type Integer))
  (if (!= Round 0)
    (set `self.Round` Round)
    (bind _aswbp_tvslide_show (cast `/Game/BluePrints/UI/Widgets/WBP_TVSlideShow` (`WidgetComponent.GetWidget` (`self.Widget`))))
    (set `TextBlock.Text` (`KismetTextLibrary.Conv_IntToText` Round) (`/Game/BluePrints/UI/Widgets/WBP_TVSlideShow.TextBlock_139` _aswbp_tvslide_show))
    (else
      (bind _aswbp_score_pop_up_effect (cast `/Game/BluePrints/UI/Widgets/WBP_ScorePopUpEffect` (`WidgetComponent.GetWidget` (`self.Widget`))))
      (set `TextBlock.Text` (`KismetTextLibrary.Conv_IntToText` (`self.Round`)) (`/Game/BluePrints/UI/Widgets/WBP_ScorePopUpEffect.TextBlock_139` _aswbp_score_pop_up_effect)))))

(fn `UserConstructionScript`)