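; BP_BasicEnvironmentLight is an environment light actor that removes itself based on the player's saved graphics setting.
; On BeginPlay it loads the "save1" slot as BP_Save and destroys itself if GraphicalSetting is one of the first two levels (0 or 1).
; It stays in the level for any other setting, or when no valid save exists.
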(event `self.ReceiveBeginPlay`
  ;[1 1 1] Save Game Logic
  (bind _returnvalue (`GameplayStatics.DoesSaveGameExist` "save1"))
  (if _returnvalue
    (bind _returnvalue_2 (`GameplayStatics.LoadGameFromSlot` "save1"))
    (bind _asbp_save (cast `/Game/BluePrints/SaveLoad/BP_Save` _returnvalue_2))
    (bind _output_get (set `self.BP Save` _asbp_save))
    (bind _graphicalsetting (`/Game/BluePrints/SaveLoad/BP_Save.GraphicalSetting` _output_get))
    (if (== _graphicalsetting 0)
      (`self.K2_DestroyActor` :!label _label)
      (elif (== _graphicalsetting 1)
        (goto _label)))))

(fn `UserConstructionScript`)