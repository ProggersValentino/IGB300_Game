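; BP_RangedEnemyBullet is a projectile, apparently fired by ranged enemies, that damages the gladiator player on contact.
; On BeginPlay it stores its forward vector as the direction, then moves along it each tick by speed with a swept location update.
; Overlapping BP_Gladiator_Player prints a debug message, sends damage through ApplyDmgMessage and destroys the bullet; other actors are ignored.
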(event `self.ReceiveBeginPlay`
  (set `self.direction` (`KismetMathLibrary.GetForwardVector` (`self.K2_GetActorRotation`))))

(event `self.ReceiveActorBeginOverlap`
  (params (OtherActor :type "Actor Object Reference"))
  (bind _asbp_gladiator_player (cast `/Game/BluePrints/GladiatorRelated/BP_Gladiator_Player` OtherActor))
  (`KismetSystemLibrary.PrintString` "Bullet Hit Player")
  (message `IPlayer.ApplyDmg` _asbp_gladiator_player (`self.damage`))
  (`self.K2_DestroyActor`))

(event `self.ReceiveTick`
  (params (DeltaSeconds :type "Float (single-precision)"))
  (`self.K2_SetActorLocation` (+ (* DeltaSeconds (`self.speed`) (`self.direction`)) (`self.K2_GetActorLocation`)) true))

(fn `UserConstructionScript`)