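; Enemy manager that assigns each enemy in its Enemies array a move target around the gladiator player inside a circular arena.
; Each tick it places targets where the player-to-enemy line meets the player's zone, using closed-form circle-circle intersection when that point falls outside the arena.
; A nested pairwise pass, rerun per enemy, nudges crowded targets apart.
; Debug circles and lines show the arena, player zone and enemy links.
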(event `self.ReceiveBeginPlay`
  (`KismetSystemLibrary.DrawDebugCircle` (0.0 0.0 0.0) 1000.0 12 (struct :`R` 1.0 :`G` 1.0 :`B` 1.0 :`A` 1.0) 100.0 10.0 (1.0 0.0 0.0) (0.0 1.0 0.0))
  (bind _returnvalue (`GameplayStatics.GetActorOfClass` "/Game/BluePrints/GladiatorRelated/BP_Gladiator_Player.BP_Gladiator_Player_C"))
  (`/Engine/EditorBlueprintResources/StandardMacros.IsValid` _returnvalue
    (:`Is Valid`
      (set `self.playerchar` _returnvalue))
    (:`Is Not Valid`
      (`KismetSystemLibrary.PrintString` "Hello"))))

(event `self.ReceiveTick`
  (params (DeltaSeconds :type "Float (single-precision)"))
  (bind _playerchar (`self.playerchar`))
  (bind _enemies (`self.enemies`))
  (bind _returnvalue (`self.K2_GetActorLocation` _playerchar))
  ;[1 1 1] Draw Player Zone
  (`/Engine/EditorBlueprintResources/StandardMacros.IsValid` _playerchar
    (:`Is Valid`
      (`KismetSystemLibrary.DrawDebugCircle` _returnvalue 300.0 12 (struct :`R` 1.0 :`G` 1.0 :`B` 1.0 :`A` 1.0) 0.0 10.0 (1.0 0.0 0.0) (0.0 1.0 0.0))
      ;[1 1 1] Calculate New Target Pos
      (for _array_element (`self.enemies`)
        (bind _returnvalue_2 (`self.K2_GetActorLocation` _array_element))
        (`KismetSystemLibrary.DrawDebugLine` _returnvalue _returnvalue_2)
        (bind _intersectpoint (`self.CircleLineIntersection` _returnvalue 300.0 _returnvalue_2 (0.0 0.0 0.0) 1000.0))
        (set `EnemyBase.targetMovePos` _intersectpoint _array_element)
        ;[1 1 1] Improve Target Move Pos Relative to Others
        (for _array_element_2 _enemies
          (for _array_element_3 _enemies
            (if (!= _array_element_2 _array_element_3)
              (bind _targetmovepos (`EnemyBase.targetMovePos` _array_element_2))
              (bind _targetmovepos_2 (`EnemyBase.targetMovePos` _array_element_3))
              (if (< (`KismetMathLibrary.Vector_Distance` _targetmovepos _targetmovepos_2) 200.0)
                (set `EnemyBase.targetMovePos` (+ _targetmovepos (* (`KismetMathLibrary.Normal` (- _targetmovepos _targetmovepos_2)) 50)) _array_element_2)))))))
    (:`Is Not Valid`
      (`KismetSystemLibrary.PrintString` "Hello"))))

(fn `CircleLineIntersection`
  (params (PlayerPos :type "Vector Structure") (ZoneR :type "Float (double-precision)") (EnemyPos :type "Vector Structure") (ArenaPos :type "Vector Structure") (ArenaR :type "Float (double-precision)"))
  (returns (IntersectPoint :type "Vector Structure"))
  (locals (a :type "Float (double-precision)") (b :type "Float (double-precision)") (q :type "Float (double-precision)"))
  (bind (_playerpos_x _playerpos_y) (`KismetMathLibrary.BreakVector` (`local.PlayerPos`)))
  (bind (_enemypos_x _enemypos_y) (`KismetMathLibrary.BreakVector` (`local.EnemyPos`)))
  (bind (_playerpos_x_2 _playerpos_y_2) (`KismetMathLibrary.BreakVector` (`local.PlayerPos`)))
  (bind (_playerpos_x_3 _playerpos_y_3) (`KismetMathLibrary.BreakVector` (`local.PlayerPos`)))
  (bind (_playerpos_x_4 _playerpos_y_4) (`KismetMathLibrary.BreakVector` (`local.PlayerPos`)))
  (bind (_playerpos_x_5 _playerpos_y_5) (`KismetMathLibrary.BreakVector` (`local.PlayerPos`)))
  (bind (_playerpos_x_6 _playerpos_y_6) (`KismetMathLibrary.BreakVector` (`local.PlayerPos`)))
  (bind (_playerpos_x_7 _playerpos_y_7) (`KismetMathLibrary.BreakVector` (`local.PlayerPos`)))
  (bind (_playerpos_x_8 _playerpos_y_8) (`KismetMathLibrary.BreakVector` (`local.PlayerPos`)))
  (bind (_arenapos_x _arenapos_y) (`KismetMathLibrary.BreakVector` (`local.ArenaPos`)))
  (bind (_playerpos_x_9 _playerpos_y_9) (`KismetMathLibrary.BreakVector` (`local.PlayerPos`)))
  (bind (_playerpos_x_10 _playerpos_y_10) (`KismetMathLibrary.BreakVector` (`local.PlayerPos`)))
  (bind _returnvalue (`KismetMathLibrary.Square` _playerpos_x_3))
  (bind _returnvalue_2 (`KismetMathLibrary.Square` _playerpos_y_3))
  (bind _returnvalue_3 (`KismetMathLibrary.Square` (`local.ZoneR`)))
  (bind _returnvalue_4 (* (`KismetMathLibrary.Square` (`local.ArenaR`)) 2.0))
  (bind _returnvalue_5 (+ PlayerPos_X (/ (* (- EnemyPos_X PlayerPos_X) ZoneR) (`KismetMathLibrary.Sqrt` (+ (`KismetMathLibrary.Square` (- EnemyPos_X PlayerPos_X)) (`KismetMathLibrary.Square` (- EnemyPos_Y PlayerPos_Y)))))))
  (bind _returnvalue_6 (+ _playerpos_y (/ (* (- _enemypos_y _playerpos_y) (`local.ZoneR`)) (`KismetMathLibrary.Sqrt` (+ (`KismetMathLibrary.Square` (- _enemypos_x _playerpos_x)) (`KismetMathLibrary.Square` (- _enemypos_y _playerpos_y)))))))
  ;[1 1 1] OutsideArena
  (if (> (+ (`KismetMathLibrary.Square` (- _returnvalue_6 _arenapos_y)) (`KismetMathLibrary.Square` (- _returnvalue_5 _arenapos_x))) (`KismetMathLibrary.Square` (`local.ArenaR`)))
    ;[1 1 1] Set quadratic sqrt
    (bind _output_get (set `local.q` (* _playerpos_y_2 (`KismetMathLibrary.Sqrt` (- (+ (* _returnvalue_4 (`KismetMathLibrary.Square` _playerpos_x_5)) (* _returnvalue_4 (`KismetMathLibrary.Square` _playerpos_y_5)) (* (`KismetMathLibrary.Square` (`local.ArenaR`)) _returnvalue_3 2.0) (* _returnvalue_3 (`KismetMathLibrary.Square` _playerpos_x_4) 2.0) (* _returnvalue_3 (`KismetMathLibrary.Square` _playerpos_y_4) 2.0)) (+ (`KismetMathLibrary.Square` _returnvalue) (* _returnvalue _returnvalue_2 2.0) (`KismetMathLibrary.Square` _returnvalue_2) (`KismetMathLibrary.Square` (`KismetMathLibrary.Square` (`local.ZoneR`))) (`KismetMathLibrary.Square` (`KismetMathLibrary.Square` (`local.ArenaR`)))))))))
    (set `local.a` (/ (- (+ _output_get (`KismetMathLibrary.MultiplyMultiply_FloatFloat` _playerpos_x_7 3.0) (* _playerpos_x_7 (`KismetMathLibrary.Square` (`local.ArenaR`))) (* (`KismetMathLibrary.Square` _playerpos_y_7) _playerpos_x_7)) (* _playerpos_x_7 (`KismetMathLibrary.Square` (`local.ZoneR`)))) (* 2.0 (+ (`KismetMathLibrary.Square` _playerpos_x_10) (`KismetMathLibrary.Square` _playerpos_y_10)))))
    (set `local.b` (/ (- (+ 0.0 (`KismetMathLibrary.MultiplyMultiply_FloatFloat` _playerpos_x_6 3.0) (* _playerpos_x_6 (`KismetMathLibrary.Square` (`local.ArenaR`))) (* (`KismetMathLibrary.Square` _playerpos_y_6) _playerpos_x_6)) (* _playerpos_x_6 (`KismetMathLibrary.Square` (`local.ZoneR`))) (`local.q`)) (* 2.0 (+ (`KismetMathLibrary.Square` _playerpos_x_9) (`KismetMathLibrary.Square` _playerpos_y_9)))))
    (if (> (* _playerpos_x_8 _playerpos_y_8) 0.0)
      (if (> _playerpos_x_8 0.0)
        (return (`KismetMathLibrary.MakeVector` (`local.b`) (`KismetMathLibrary.Sqrt` (- (`KismetMathLibrary.Square` (`local.ArenaR`)) (`KismetMathLibrary.Square` (`local.b`))))))
        (else
          (return (`KismetMathLibrary.MakeVector` (`local.b`) (* (`KismetMathLibrary.Sqrt` (- (`KismetMathLibrary.Square` (`local.ArenaR`)) (`KismetMathLibrary.Square` (`local.b`)))) -1.0)))))
      (elif (> _playerpos_x_8 0.0)
        (return (`KismetMathLibrary.MakeVector` (`local.a`)))
        (else
          (return (`KismetMathLibrary.MakeVector` (`local.a`) (`KismetMathLibrary.Sqrt` (- (`KismetMathLibrary.Square` (`local.ArenaR`)) (`KismetMathLibrary.Square` (`local.a`)))))))))
    (else
      (return (`KismetMathLibrary.MakeVector` _returnvalue_5 _returnvalue_6)))))

(fn `UserConstructionScript`)