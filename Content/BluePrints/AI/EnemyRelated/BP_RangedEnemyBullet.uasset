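; BP_RangedEnemyBullet is the projectile thrown by a ranged enemy, which reports hits on the player back to its thrower.
; It caches its forward vector at BeginPlay and moves along it each Tick with a swept location update.
; On overlapping the player, it sends the Event.Montage.Throw gameplay event to the thrower with the player as target data, leaving the hit response to that actor, then destroys itself.
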(event `self.ReceiveActorBeginOverlap`
  (params (OtherActor :type "Actor Object Reference"))
  (bind _enemythatthrew (`self.EnemyThatThrew`))
  (cast `/Game/BluePrints/Player/GladiatorRelated/BP_WWEGladiator_Player` OtherActor)
  (`AbilitySystemBlueprintLibrary.SendGameplayEventToActor` _enemythatthrew (struct :`TagName` "Event.Montage.Throw") (make `GameplayEventData` (struct) _enemythatthrew OtherActor null null (struct) (struct) (struct) 0.0 (`AbilitySystemBlueprintLibrary.AbilityTargetDataFromActor` OtherActor)))
  (`self.K2_DestroyActor`))

(event `self.ReceiveBeginPlay`
  (set `self.direction` (`KismetMathLibrary.GetForwardVector` (`self.K2_GetActorRotation`))))

(event `self.ReceiveTick`
  (params (DeltaSeconds :type "Float (single-precision)"))
  (`self.K2_SetActorLocation` (+ (* DeltaSeconds (`self.speed`) (`self.direction`)) (`self.K2_GetActorLocation`)) true))

(fn `UserConstructionScript`)