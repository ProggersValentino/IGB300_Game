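; Enemy manager that runs arena combat waves and steers enemies around the gladiator player.
; When no enemies remain, it spawns melee enemies at random spawn locations by wave difficulty, pausing between rounds.
; Each tick it sets move targets from a zone around the player, pushes close targets apart and controls facing.
; Fear widens the zone and turns enemies away; random group attacks and the C++ spawner are disconnected, marked deprecated.
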(event `self.ReceiveBeginPlay`
  (bind _returnvalue (`GameplayStatics.GetActorOfClass` "/Game/BluePrints/Player/GladiatorRelated/BP_WWEGladiator_Player.BP_WWEGladiator_Player_C"))
  (`/Engine/EditorBlueprintResources/StandardMacros.IsValid` _returnvalue
    (:`Is Valid`
      (set `self.playerchar` _returnvalue))
    (:`Is Not Valid`
      (`KismetSystemLibrary.PrintString` "ERROR: Player not set on enemy manager, possible race condition"))))

(event `self.ReceiveTick`
  (params (DeltaSeconds :type "Float (single-precision)"))
  (bind _playerchar (`self.playerchar`))
  (bind _playerchar_2 (`self.playerchar`))
  (bind _enemiesfearing (`self.EnemiesFearing`))
  (bind _enemies (`self.enemies`))
  (bind (_returnvalue_x _returnvalue_y) (`KismetMathLibrary.BreakVector` (`self.K2_GetActorLocation` _playerchar_2)))
  (`KismetSystemLibrary.PrintString` "firing")
  (if (and (`self.EnemiesFearingLast`) _enemiesfearing)
    _
    (elif _enemiesfearing
      (`self.Event Fearing Start`)
      (else
        (`self.Event Fearing End`))))
  ;[1 1 1] Infinte Spawning Wave 0
  (if (and (== (`KismetArrayLibrary.Array_Length` (`self.enemies`)) 0) (!= (`KismetArrayLibrary.Array_Length` (`self.waves`)) 0))
    (if (not (`self.IsDelayingForNextRound`))
      ;[1 1 1] End of round
      (if (`self.IsFirstWave?`)
        (set `self.IsFirstWave?` false)
        (`self.SpawnFromDifficulty`)
        (else
          (`KismetSystemLibrary.PrintString` "Waiting for next round..." true true (struct :`R` 0.134947 :`G` 1.0 :`A` 1.0))
          (set `self.IsDelayingForNextRound` true)
          (`KismetSystemLibrary.Delay` 1.0)
          (`self.EngageEndOfRound`)
          (`KismetSystemLibrary.Delay` (`self.NextRoundDelay`))
          (`self.SpawnFromDifficulty`)
          (set `self.IsDelayingForNextRound` false))))
    (else
      (`/Engine/EditorBlueprintResources/StandardMacros.IsValid` (`self.playerchar`)
        (:`Is Valid`
          ;[1 1 1] Calculate New Target Pos
          (for _array_element (`self.enemies`)
            (if (and (`KismetSystemLibrary.IsValid` _array_element) (`KismetSystemLibrary.IsValid` _playerchar))
              (set `EnemyBase.targetMovePos` (`self.TargetEnemyPositionCalculator` (`self.K2_GetActorLocation` _playerchar) (`self.K2_GetActorLocation` _array_element) (0.0 0.0 0.0) (`self.ZoneSize`) 1500.0) _array_element)
              ;[1 1 1] Improve Target Move Pos Relative to Others
              (for _array_element_2 _enemies
                (for _array_element_3 _enemies
                  (if (!= _array_element_2 _array_element_3)
                    (bind _targetmovepos (`EnemyBase.targetMovePos` _array_element_2))
                    (bind _targetmovepos_2 (`EnemyBase.targetMovePos` _array_element_3))
                    (if (< (`KismetMathLibrary.Vector_Distance` _targetmovepos _targetmovepos_2) 200.0)
                      (set `EnemyBase.targetMovePos` (+ _targetmovepos (* (`KismetMathLibrary.Normal` (- _targetmovepos _targetmovepos_2)) 50)) _array_element_2)))))
              ;[1 1 1] Make enemies face player (should move this to c++)
              (for _array_element_4 (`self.enemies`)
                (if (`KismetSystemLibrary.IsValid` _playerchar_2)
                  (if (`self.EnemiesFearing`)
                    (bind (_returnvalue_x_2 _returnvalue_y_2) (`KismetMathLibrary.BreakVector` (`self.K2_GetActorLocation` _array_element_4)))
                    (`self.K2_SetActorRotation` _array_element_4 (`KismetMathLibrary.FindLookAtRotation` (`KismetMathLibrary.MakeVector` _returnvalue_x _returnvalue_y) (`KismetMathLibrary.MakeVector` _returnvalue_x_2 _returnvalue_y_2)) false)
                    (else
                      (`self.K2_SetActorRotation` _array_element_4 (`KismetMathLibrary.FindLookAtRotation` (`KismetMathLibrary.MakeVector` _returnvalue_x_2 _returnvalue_y_2) (`KismetMathLibrary.MakeVector` _returnvalue_x _returnvalue_y)) false))))))))
        (:`Is Not Valid`
          (`KismetSystemLibrary.PrintString` "Player died - fweaking idiot")
          (`self.K2_DestroyActor`))))))

(event `Event Fearing Start`
  (for _array_element (`self.enemies`)
    (bind _asbp_basic_melee_enemy (cast `/Game/BluePrints/AI/EnemyRelated/Enemies/BP_BasicMeleeEnemy` _array_element))
    (set `/Game/BluePrints/AI/EnemyRelated/Enemies/BP_BasicMeleeEnemy.Fearing` true _asbp_basic_melee_enemy)
    (set `self.ZoneSize` 600.0)
    (set `self.EnemiesFearingLast` true)))

(event `Event Fearing End`
  (for _array_element (`self.enemies`)
    (bind _asbp_basic_melee_enemy (cast `/Game/BluePrints/AI/EnemyRelated/Enemies/BP_BasicMeleeEnemy` _array_element))
    (set `/Game/BluePrints/AI/EnemyRelated/Enemies/BP_BasicMeleeEnemy.Fearing` false _asbp_basic_melee_enemy)
    (set `self.ZoneSize` 300.0)
    (set `self.EnemiesFearingLast` false)))

(fn `CircleLineIntersection`
  (params (PlayerPos :type "Vector Structure") (ZoneR :type "Float (double-precision)") (EnemyPos :type "Vector Structure") (ArenaPos :type "Vector Structure") (ArenaR :type "Float (double-precision)"))
  (returns (IntersectPoint :type "Vector Structure"))
  (locals (a :type "Float (double-precision)") (b :type "Float (double-precision)") (q :type "Float (double-precision)"))
  (bind (_playerpos_x _playerpos_y) (`KismetMathLibrary.BreakVector` (`local.PlayerPos`)))
  (bind (_enemypos_x _enemypos_y) (`KismetMathLibrary.BreakVector` (`local.EnemyPos`)))
  (bind (_playerpos_x_2 _playerpos_y_2) (`KismetMathLibrary.BreakVector` (`local.PlayerPos`)))
  (bind (_playerpos_x_3 _playerpos_y_3) (`KismetMathLibrary.BreakVector` (`local.PlayerPos`)))
  (bind (_playerpos_x_4 _playerpos_y_4) (`KismetMathLibrary.BreakVector` (`local.PlayerPos`)))
  (bind (_playerpos_x_5 _playerpos_y_5) (`KismetMathLibrary.BreakVector` (`local.PlayerPos`)))
  (bind (_playerpos_x_6 _playerpos_y_6) (`KismetMathLibrary.BreakVector` (`local.PlayerPos`)))
  (bind (_playerpos_x_7 _playerpos_y_7) (`KismetMathLibrary.BreakVector` (`local.PlayerPos`)))
  (bind (_playerpos_x_8 _playerpos_y_8) (`KismetMathLibrary.BreakVector` (`local.PlayerPos`)))
  (bind (_arenapos_x _arenapos_y) (`KismetMathLibrary.BreakVector` (`local.ArenaPos`)))
  (bind (_playerpos_x_9 _playerpos_y_9) (`KismetMathLibrary.BreakVector` (`local.PlayerPos`)))
  (bind (_playerpos_x_10 _playerpos_y_10) (`KismetMathLibrary.BreakVector` (`local.PlayerPos`)))
  (bind _returnvalue (`KismetMathLibrary.Square` _playerpos_x_3))
  (bind _returnvalue_2 (`KismetMathLibrary.Square` _playerpos_y_3))
  (bind _returnvalue_3 (`KismetMathLibrary.Square` (`local.ZoneR`)))
  (bind _returnvalue_4 (* (`KismetMathLibrary.Square` (`local.ArenaR`)) 2.0))
  (bind _returnvalue_5 (+ PlayerPos_X (/ (* (- EnemyPos_X PlayerPos_X) ZoneR) (`KismetMathLibrary.Sqrt` (+ (`KismetMathLibrary.Square` (- EnemyPos_X PlayerPos_X)) (`KismetMathLibrary.Square` (- EnemyPos_Y PlayerPos_Y)))))))
  (bind _returnvalue_6 (+ _playerpos_y (/ (* (- _enemypos_y _playerpos_y) (`local.ZoneR`)) (`KismetMathLibrary.Sqrt` (+ (`KismetMathLibrary.Square` (- _enemypos_x _playerpos_x)) (`KismetMathLibrary.Square` (- _enemypos_y _playerpos_y)))))))
  ;[1 1 1] OutsideArena
  (if (> (+ (`KismetMathLibrary.Square` (- _returnvalue_6 _arenapos_y)) (`KismetMathLibrary.Square` (- _returnvalue_5 _arenapos_x))) (`KismetMathLibrary.Square` (`local.ArenaR`)))
    ;[1 1 1] Set quadratic sqrt
    (bind _output_get (set `local.q` (* _playerpos_y_2 (`KismetMathLibrary.Sqrt` (- (+ (* _returnvalue_4 (`KismetMathLibrary.Square` _playerpos_x_5)) (* _returnvalue_4 (`KismetMathLibrary.Square` _playerpos_y_5)) (* (`KismetMathLibrary.Square` (`local.ArenaR`)) _returnvalue_3 2.0) (* _returnvalue_3 (`KismetMathLibrary.Square` _playerpos_x_4) 2.0) (* _returnvalue_3 (`KismetMathLibrary.Square` _playerpos_y_4) 2.0)) (+ (`KismetMathLibrary.Square` _returnvalue) (* _returnvalue _returnvalue_2 2.0) (`KismetMathLibrary.Square` _returnvalue_2) (`KismetMathLibrary.Square` (`KismetMathLibrary.Square` (`local.ZoneR`))) (`KismetMathLibrary.Square` (`KismetMathLibrary.Square` (`local.ArenaR`)))))))))
    (set `local.a` (/ (- (+ _output_get (`KismetMathLibrary.MultiplyMultiply_FloatFloat` _playerpos_x_7 3.0) (* _playerpos_x_7 (`KismetMathLibrary.Square` (`local.ArenaR`))) (* (`KismetMathLibrary.Square` _playerpos_y_7) _playerpos_x_7)) (* _playerpos_x_7 (`KismetMathLibrary.Square` (`local.ZoneR`)))) (* 2.0 (+ (`KismetMathLibrary.Square` _playerpos_x_10) (`KismetMathLibrary.Square` _playerpos_y_10)))))
    (set `local.b` (/ (- (+ 0.0 (`KismetMathLibrary.MultiplyMultiply_FloatFloat` _playerpos_x_6 3.0) (* _playerpos_x_6 (`KismetMathLibrary.Square` (`local.ArenaR`))) (* (`KismetMathLibrary.Square` _playerpos_y_6) _playerpos_x_6)) (* _playerpos_x_6 (`KismetMathLibrary.Square` (`local.ZoneR`))) (`local.q`)) (* 2.0 (+ (`KismetMathLibrary.Square` _playerpos_x_9) (`KismetMathLibrary.Square` _playerpos_y_9)))))
    (if (> (* _playerpos_x_8 _playerpos_y_8) 0.0)
      (if (> _playerpos_x_8 0.0)
        (return (`KismetMathLibrary.MakeVector` (`local.b`) (`KismetMathLibrary.Sqrt` (- (`KismetMathLibrary.Square` (`local.ArenaR`)) (`KismetMathLibrary.Square` (`local.b`))))))
        (else
          (return (`KismetMathLibrary.MakeVector` (`local.b`) (* (`KismetMathLibrary.Sqrt` (- (`KismetMathLibrary.Square` (`local.ArenaR`)) (`KismetMathLibrary.Square` (`local.b`)))) -1.0)))))
      (elif (> _playerpos_x_8 0.0)
        (return (`KismetMathLibrary.MakeVector` (`local.a`)))
        (else
          (return (`KismetMathLibrary.MakeVector` (`local.a`) (`KismetMathLibrary.Sqrt` (- (`KismetMathLibrary.Square` (`local.ArenaR`)) (`KismetMathLibrary.Square` (`local.a`)))))))))
    (else
      (return (`KismetMathLibrary.MakeVector` _returnvalue_5 _returnvalue_6)))))

(fn `EnemyGroupAttack`
  (params (Enemies :type "Array of EnemyBase Object Reference (by ref)") (enemyType :type "EEnemyType Enum" :default "ET_Basic"))
  (locals (i :type Integer))
  (switch `EEnemyType` enemyType
    (:`ET_Basic`
      (for _array_element Enemies
        (bind _returnvalue (`EnemyBase.IsOfType` _array_element))
        (if (`|EnumEquality` _returnvalue "ET_Basic")
          (`IEnemy.Attack` _array_element)
          (bind _result (`/Engine/EditorBlueprintResources/StandardMacros.IncrementInt` (`local.i`))
            (:`  `
              (if (>= _result (`KismetMathLibrary.RandomIntegerInRange` (`self.minMeleeAttacking`) (`self.maxMeleeAttacking`)))
                (break))))))
      (return))
    (:`ET_Ranged`
      (for _array_element_2 Enemies
        (bind _returnvalue_2 (`EnemyBase.IsOfType` _array_element_2))
        (if (`|EnumEquality` _returnvalue_2 "ET_Ranged")
          (`IEnemy.Attack` _array_element_2)
          (bind _result_2 (`/Engine/EditorBlueprintResources/StandardMacros.IncrementInt` (`local.i`))
            (:`  `
              (if (>= _result_2 (`KismetMathLibrary.RandomIntegerInRange` (`self.minRangedAttacking`) (`self.maxRangedAttacking`)))
                (break))))))
      (return))
    (:`ET_Tank`
      (for _array_element_3 Enemies
        (bind _returnvalue_3 (`EnemyBase.IsOfType` _array_element_3))
        (if (`|EnumEquality` _returnvalue_3 "ET_Tank")
          (`IEnemy.Attack` _array_element_3)
          (bind _result_3 (`/Engine/EditorBlueprintResources/StandardMacros.IncrementInt` (`local.i`))
            (:`  `
              (if (>= _result_3 (`KismetMathLibrary.RandomIntegerInRange` (`self.minTankAttacking`) (`self.maxTankAttacking`)))
                (break))))))
      (return))))

(fn `SpawnFromDifficulty`
  (locals (spawnLocIndex :type Integer) (location :type "Vector Structure"))
  (bind (_value _returnvalue) (`BlueprintMapLibrary.Map_Find` (`self.spawnLocations`) (`KismetMathLibrary.RandomInteger` (`BlueprintMapLibrary.Map_Length` (`self.spawnLocations`)))))
  (if (> (`BlueprintMapLibrary.Map_Length` (`self.spawnLocations`)) 0)
    (for _ (range 1 (+ (`KismetMathLibrary.FFloor` (`self.WaveDifficulty`)) 1))
      (if _returnvalue
        (bind _output_get (set `local.location` _value))
        (`|SpawnActorFromClass` "/Game/BluePrints/AI/EnemyRelated/Enemies/BP_BasicMeleeEnemy.BP_BasicMeleeEnemy_C" (`KismetMathLibrary.MakeTransform` _output_get) "Undefined" "MultiplyWithRoot" null null)
        (else
          (`KismetSystemLibrary.PrintString` "Error Finding Spawn Location Element"))))
    (return)
    (else
      (`KismetSystemLibrary.PrintString` "No Spawn Locations present for spawning"))))

(fn `UserConstructionScript`)