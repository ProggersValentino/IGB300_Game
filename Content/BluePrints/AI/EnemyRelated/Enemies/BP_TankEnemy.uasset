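; Tank enemy Blueprint that defines a GAS-driven melee attack against the gladiator player.
; Attack activates GA_Melee, then sphere-traces for pawns along the enemy's forward vector at a fixed world height, using AttackRange and AttackRadius.
; If the hit is the player, it sends itself a slash montage gameplay event carrying that actor as target data.
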(event `self.ReceiveTick`
  (params (DeltaSeconds :type "Float (single-precision)")))

(event `self.Attack`
  (bind (_returnvalue_location _returnvalue_rotation) (`KismetMathLibrary.BreakTransform` (`self.GetTransform`)))
  (bind _returnvalue (`KismetMathLibrary.MakeVector` (.x _returnvalue_location) (.y _returnvalue_location) 100.0))
  (bind _returnvalue_2 (`AbilitySystemComponent.TryActivateAbilityByClass` (`AbilitySystemBlueprintLibrary.GetAbilitySystemComponent` null) "/Game/BluePrints/AI/EnemyRelated/Abilities/GA_Melee.GA_Melee_C" true))
  (if _returnvalue_2
    (bind _outhit (`KismetSystemLibrary.SphereTraceSingleForObjects` _returnvalue (+ _returnvalue (* (`KismetMathLibrary.GetForwardVector` _returnvalue_rotation) (`self.AttackRange`))) (`self.AttackRadius`) (`|MakeArray` "ObjectTypeQuery3" :!type "EObjectTypeQuery Enum")))
    (cast `/Game/BluePrints/Player/GladiatorRelated/BP_Gladiator_Player` (`.HitActor` (`GameplayStatics.BreakHitResult` _outhit)))
    (`AbilitySystemBlueprintLibrary.SendGameplayEventToActor` self (struct :`TagName` "Event.Montage.Slash") (make `GameplayEventData` (struct) self (`.HitActor` (`GameplayStatics.BreakHitResult` _outhit)) null null (struct) (struct) (struct) 0.0 (`AbilitySystemBlueprintLibrary.AbilityTargetDataFromActor` (`.HitActor` (`GameplayStatics.BreakHitResult` _outhit)))))))

(fn `UserConstructionScript`)