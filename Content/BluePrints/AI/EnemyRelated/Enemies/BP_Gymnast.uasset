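; BP_Gymnast is a melee enemy that attacks the gladiator player and reacts to blocks and hits.
; Attack line-traces toward the EnemySubsystem's player position, classifies the hit as front or back by dot product, tags itself and sends a slash gameplay event carrying the target.
; Block plays a recoil montage, while Damage plays a hit montage and holds a stun flag until a recovery delay ends.
; Construction enables custom-depth stencil rendering.
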(event `self.Attack`
  (bind _returnvalue_location (`KismetMathLibrary.BreakTransform` (`self.GetTransform`)))
  (bind _returnvalue (`KismetMathLibrary.MakeVector` (.x _returnvalue_location) (.y _returnvalue_location) 150.0))
  (bind _returnvalue_2 (`EnemySubsystem.RequestPlayerPosition` (subsystem `EnemySubsystem`)))
  (bind _outhit (`KismetSystemLibrary.LineTraceSingleForObjects` :`Start` _returnvalue :`End` (+ _returnvalue (* (`KismetMathLibrary.Normal` (- _returnvalue_2 _returnvalue_location)) (`self.AttackRange`))) :`ObjectTypes` (`|MakeArray` "ObjectTypeQuery3" :!type "EObjectTypeQuery Enum") :`DrawDebugType` "ForDuration"))
  (bind _asbp_wwegladiator_player (cast `/Game/BluePrints/Player/GladiatorRelated/BP_WWEGladiator_Player` (`.HitActor` (`GameplayStatics.BreakHitResult` _outhit))))
  (bind _directiontag (`self.Get Hit Direction` (`self.K2_GetActorLocation`) (`self.K2_GetActorLocation` _asbp_wwegladiator_player) (`self.GetActorForwardVector` _asbp_wwegladiator_player)))
  (bind _returnvalue_3 (`BlueprintGameplayTagLibrary.MakeGameplayTagContainerFromTag` _directiontag))
  (`AbilitySystemBlueprintLibrary.AddLooseGameplayTags` self _returnvalue_3) ; adding a tempory tag to enemy of whether its hitting the player\nfrom behind or infront
  (`AbilitySystemBlueprintLibrary.SendGameplayEventToActor` self (struct :`TagName` "Event.Montage.Slash") (make `GameplayEventData` (struct) self (`.HitActor` (`GameplayStatics.BreakHitResult` _outhit)) null null (struct) (struct) _returnvalue_3 0.0 (`AbilitySystemBlueprintLibrary.AbilityTargetDataFromActor` (`.HitActor` (`GameplayStatics.BreakHitResult` _outhit))))))

(event `self.Block`
  (`|PlayMontage` (`self.Mesh`) (`self.BlockRecoilReaction`)))

(event `self.Damage`
  (params (amount :type "Float (single-precision)"))
  ;[1 1 1] Play animation when hit
  (`|PlayMontage` (`self.Mesh`) (`self.Attacked_Animation`) (`self.StunAnimationSpeed`)
    (:`then`
      (set `self.b_IsStunned` true))
    (:`OnCompleted`
      (`KismetSystemLibrary.Delay` (`self.StunRecoveryTime`))
      (set `self.b_IsStunned` false))))

(fn `Get Hit Direction`
  (params (`Owner Loco` :type "Vector Structure") (`Target Loco` :type "Vector Structure") (`Target Forward Vec` :type "Vector Structure"))
  (returns (DirectionTag :type "GameplayTag Structure"))
  (locals (AngleTolerance :type "Float (double-precision)" :default 110.0))
  (if (> (`KismetMathLibrary.Dot_VectorVector` `Target Forward Vec` (`KismetMathLibrary.Normal` (- `Owner Loco` `Target Loco`))) (`KismetMathLibrary.Cos` (* (`local.AngleTolerance`) 0.5)))
    (return (struct :`TagName` "Gameplay.HitDirection.Forward"))
    (else
      (return (struct :`TagName` "Gameplay.HitDirection.Backward")))))

(fn `UserConstructionScript`
  (bind _mesh (`self.Mesh`))
  (`PrimitiveComponent.SetRenderCustomDepth` _mesh true)
  (`PrimitiveComponent.SetCustomDepthStencilValue` _mesh (`self.Stencil`)))