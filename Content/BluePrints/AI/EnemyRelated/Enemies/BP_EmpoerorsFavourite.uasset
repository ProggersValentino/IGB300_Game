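; Enemy gladiator Blueprint for the Emperor's Favourite, which taunts, attacks the player, reacts to hits and blocks, and rewards kills.
; Attack line-traces for the player, tags a front or back hit by dot product, and sends a GAS slash event.
; Damage plays a stun montage with Niagara VFX; death updates kill stats and spawns score and coin actors.
; Tick calls the taunt montage, while look-at movement and health-based outline code are disconnected.
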(event `self.ReceiveTick`
  (params (DeltaSeconds :type "Float (single-precision)"))
  (`|PlayMontage` (`self.Mesh`) "/Game/BluePrints/Player/GladiatorRelated/Anim/Mixamo/AM_Taunt.AM_Taunt"
    (:`OnCompleted`
      _)
    (:`OnBlendOut`
      _)
    (:`OnInterrupted`
      _)
    (:`OnNotifyBegin`
      _)
    (:`OnNotifyEnd`
      _))
  (`KismetSystemLibrary.Delay` 3.0))

(event `self.Attack`
  (bind (_returnvalue_location _returnvalue_rotation) (`KismetMathLibrary.BreakTransform` (`self.GetTransform`)))
  (bind _returnvalue (`KismetMathLibrary.MakeVector` (.x _returnvalue_location) (.y _returnvalue_location) 100.0))
  (bind _outhit (`KismetSystemLibrary.LineTraceSingleForObjects` _returnvalue (+ _returnvalue (* (`KismetMathLibrary.GetForwardVector` _returnvalue_rotation) (`self.AttackRange`))) (`|MakeArray` "ObjectTypeQuery3" :!type "EObjectTypeQuery Enum")))
  (bind _asbp_wwegladiator_player (cast `/Game/BluePrints/Player/GladiatorRelated/BP_WWEGladiator_Player` (`.HitActor` (`GameplayStatics.BreakHitResult` _outhit))))
  (bind _directiontag (`self.GetHitDirection` (`self.K2_GetActorLocation`) (`self.K2_GetActorLocation` _asbp_wwegladiator_player) (`self.GetActorForwardVector` _asbp_wwegladiator_player)))
  (bind _returnvalue_2 (`BlueprintGameplayTagLibrary.MakeGameplayTagContainerFromTag` _directiontag))
  (`AbilitySystemBlueprintLibrary.AddLooseGameplayTags` self _returnvalue_2) ; adding a tempory tag to enemy of whether its hitting the player\nfrom behind or infront
  (`AbilitySystemBlueprintLibrary.SendGameplayEventToActor` self (struct :`TagName` "Event.Montage.Slash") (make `GameplayEventData` (struct) self (`.HitActor` (`GameplayStatics.BreakHitResult` _outhit)) null null (struct) (struct) _returnvalue_2 0.0 (`AbilitySystemBlueprintLibrary.AbilityTargetDataFromActor` (`.HitActor` (`GameplayStatics.BreakHitResult` _outhit))))))

(event `self.Damage`
  (params (amount :type "Float (single-precision)"))
  ;[1 1 1] Play animation when hit
  (`|PlayMontage` (`self.Mesh`) (`self.Attacked_Animation`) (`self.StunAnimationSpeed`)
    (:`then`
      (`KismetSystemLibrary.DelayUntilNextTick`)
      (set `self.Stunned` true)
      ;[1 1 1] Turn On And Off VFX
      (`ActorComponent.Activate` (`self.Niagara`) true))
    (:`OnBlendOut`
      (set `self.Stunned` false :!label _label))
    (:`OnInterrupted`
      (goto _label))))

(event `self.PostDeathAction`
  (bind _returnvalue (`KismetMathLibrary.Conv_VectorToTransform` (- (`self.K2_GetActorLocation`) (0.0 0.0 90.0))))
  ;[0.899 1 0.2475] Increase Total kill counter
  (set `self.IsDead` true)
  (`GameplayStats.ChangeTotalKills` (subsystem `GameplayStats`) 1)
  (`|SpawnActorFromClass` "/Game/BluePrints/UI/Widgets/BP_ScorePopUp.BP_ScorePopUp_C" _returnvalue "Undefined" "MultiplyWithRoot" null null)
  (`|SpawnActorFromClass` "/Game/VFX/SpawnBPs/BP_CoinFountain.BP_CoinFountain_C" _returnvalue "Undefined" "MultiplyWithRoot" null null))

(event `self.Block`
  (`|PlayMontage` (`self.Mesh`) (`self.BlockRecoilReaction`)))

(fn `GetHitDirection`
  (params (OwnerLoco :type "Vector Structure") (TargetLoco :type "Vector Structure") (TargetForwardVec :type "Vector Structure"))
  (returns (DirectionTag :type "GameplayTag Structure"))
  (locals (AngleTolerance :type "Float (double-precision)" :default 110.0))
  ;[1 1 1] To determine what direction the enemy is hitting the player at and whether if its at the front or the back
  (if (> (`KismetMathLibrary.Dot_VectorVector` TargetForwardVec (`KismetMathLibrary.Normal` (- OwnerLoco TargetLoco))) (`KismetMathLibrary.Cos` (* (`local.AngleTolerance`) 0.5)))
    (return (struct :`TagName` "Gameplay.HitDirection.Forward"))
    (else
      (return (struct :`TagName` "Gameplay.HitDirection.Backward")))))

(fn `IsCloseToTarget`
  (returns (Close :type Boolean))
  (return (< (`KismetMathLibrary.Vector_Distance` (`self.K2_GetActorLocation`) (`self.targetMovePos`)) (`self.IsCloseToTargetLimit`))))

(fn `UserConstructionScript`
  (bind _mesh (`self.Mesh`))
  (`PrimitiveComponent.SetRenderCustomDepth` _mesh true)
  (`PrimitiveComponent.SetCustomDepthStencilValue` _mesh (`self.Stencil`)))