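; BP_DebugEnemyMove is a debug enemy actor that moves in a straight line toward a Targetpos location.
; Each Tick it steps along the normalized direction by Speed, a per-frame distance not scaled by delta time.
; If that step would end farther from the target than the current location, it snaps to Targetpos instead.
; Movement uses SetActorLocation without sweep, and nothing in these graphs sets the target.
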(event `self.ReceiveTick`
  (params (DeltaSeconds :type "Float (single-precision)"))
  (bind _returnvalue (`self.K2_GetActorLocation`))
  (bind _targetpos (`self.targetpos`))
  (bind _returnvalue_2 (+ (* (`KismetMathLibrary.Normal` (- _targetpos _returnvalue)) (`self.speed`)) _returnvalue))
  (if (> (`KismetMathLibrary.Vector_Distance` _returnvalue_2 _targetpos) (`KismetMathLibrary.Vector_Distance` _returnvalue _targetpos))
    (`self.K2_SetActorLocation` (`self.targetpos`))
    (else
      (`self.K2_SetActorLocation` _returnvalue_2))))

(fn `UserConstructionScript`)