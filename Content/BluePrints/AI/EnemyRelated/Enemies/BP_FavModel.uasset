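; BP_FavModel is a character that stays in place and repeatedly plays a WWE taunt montage.
; BeginPlay disables movement and starts the montage, whose callbacks all feed a three-second delay that replays it through the Play event.
; The construction script enables custom depth with a configurable stencil value on the mesh.
; A dot-product helper classifies hit direction as forward or backward, but nothing here calls it.
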(event `self.ReceiveBeginPlay`
  (`CharacterMovementComponent.DisableMovement` (`self.CharacterMovement`))
  (`|PlayMontage` (`self.Mesh`) "/Game/BluePrints/Player/GladiatorRelated/Anim/Animations/NewAnimBlueprints/AM_WWE_Taunt_Final.AM_WWE_Taunt_Final"
    (:`OnCompleted`
      _)
    (:`OnBlendOut`
      _)
    (:`OnInterrupted`
      _)
    (:`OnNotifyBegin`
      _)
    (:`OnNotifyEnd`
      _))
  (`KismetSystemLibrary.Delay` 3.0)
  (`self.Play`))

(event `self.ReceiveTick`
  (params (DeltaSeconds :type "Float (single-precision)")))

(event `Play`
  (`|PlayMontage` (`self.Mesh`) "/Game/BluePrints/Player/GladiatorRelated/Anim/Animations/NewAnimBlueprints/AM_WWE_Taunt_Final.AM_WWE_Taunt_Final"
    (:`OnCompleted`
      _)
    (:`OnBlendOut`
      _)
    (:`OnInterrupted`
      _)
    (:`OnNotifyBegin`
      _)
    (:`OnNotifyEnd`
      _))
  (`KismetSystemLibrary.Delay` 3.0)
  (`self.Play`))

(fn `GetHitDirection`
  (params (OwnerLoco :type "Vector Structure") (TargetLoco :type "Vector Structure") (TargetForwardVec :type "Vector Structure"))
  (returns (DirectionTag :type "GameplayTag Structure"))
  (locals (AngleTolerance :type "Float (double-precision)" :default 110.0))
  ;[1 1 1] To determine what direction the enemy is hitting the player at and whether if its at the front or the back
  (if (> (`KismetMathLibrary.Dot_VectorVector` TargetForwardVec (`KismetMathLibrary.Normal` (- OwnerLoco TargetLoco))) (`KismetMathLibrary.Cos` (* (`local.AngleTolerance`) 0.5)))
    (return (struct :`TagName` "Gameplay.HitDirection.Forward"))
    (else
      (return (struct :`TagName` "Gameplay.HitDirection.Backward")))))

(fn `UserConstructionScript`
  (bind _mesh (`self.Mesh`))
  (`PrimitiveComponent.SetRenderCustomDepth` _mesh true)
  (`PrimitiveComponent.SetCustomDepthStencilValue` _mesh (`self.Stencil`)))