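; BP_Crowd is the arena crowd that reacts to how entertaining the gladiator player is and can reward thrown items.
; Each tick it raises or slowly decays excitement in CrowdWorldSubsystem, grows crowd size, and feeds the audio manager, VFX controller and bar flash.
; Full excitement triggers the item UI once; ThrowBall, when the crowd is primed, has the spawner throw an item and resets excitement.
; Coin increases also go to the subsystem.
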(event `self.ReceiveBeginPlay`
  (bind _returnvalue (`GameplayStatics.GetActorOfClass` "/Game/Audio/BP_AudioManager.BP_AudioManager_C"))
  (set `self.AudioManager` _returnvalue)
  (`ActorComponent.Deactivate` (`Actor.RootComponent` (`self.CoinEffect`)))
  (set `self.CoinsActive` false)
  (bind _returnvalue_2 (`GameplayStatics.GetActorOfClass` "/Game/BluePrints/Player/GladiatorRelated/BP_WWEGladiator_Player.BP_WWEGladiator_Player_C"))
  (set `self.Player` _returnvalue_2)
  (bind _returnvalue_3 (`GameplayStatics.GetActorOfClass` "/Game/BluePrints/InteractableSystem/BP_Spawn_Item.BP_Spawn_Item_C"))
  (set `self.Spawner` _returnvalue_3)
  (bind _returnvalue_4 (`GameplayStatics.GetActorOfClass` "/Game/BluePrints/GlorySystem/CrowdVFX/BP_VFXCrowdController.BP_VFXCrowdController_C"))
  (set `self.Crowd VFX Controller` _returnvalue_4))

(event `self.ReceiveTick`
  (params (DeltaSeconds :type "Float (single-precision)"))
  (bind _returnvalue (subsystem `CrowdWorldSubsystem`))
  (bind _returnvalue_2 (subsystem `CrowdWorldSubsystem`))
  (bind _returnvalue_3 (+ (`CrowdWorldSubsystem.GetCrowdSize` _returnvalue) 1))
  (if (`/Game/BluePrints/Player/GladiatorRelated/BP_WWEGladiator_Player.IsEntertaining` (`self.Player`))
    (`self.BarFlash`)
    (`self.UpdateCrowd` (* DeltaSeconds 15.0))
    (`CrowdWorldSubsystem.SetCrowdSize` _returnvalue _returnvalue_3)
    (bind _returnvalue_4 (`GameplayStatics.GetActorOfClass` "/Game/BluePrints/GlorySystem/CrowdVFX/BP_VFXCrowdController.BP_VFXCrowdController_C"))
    (set `/Game/BluePrints/GlorySystem/CrowdVFX/BP_VFXCrowdController.CurrentCrowdSize` (`KismetMathLibrary.Conv_IntToDouble` _returnvalue_3) _returnvalue_4)
    (else
      (`self.BarOff`)
      (`self.UpdateCrowd` (* DeltaSeconds -0.5))))
  ;[1 1 1] State Machine
  (if (and (>= (`CrowdWorldSubsystem.GetExcitement` _returnvalue_2) (`CrowdWorldSubsystem.GetMaxExcitement` _returnvalue_2)) (not (`self.itemcalled`)))
    (`self.ActivateItemUI`)
    (set `self.itemcalled` true)
    (else
      (`KismetSystemLibrary.PrintString` "Other states handles by AudioManager" false false))))

(event `Increase Coin Counter`
  (params (`Coin Increase` :type Integer))
  (`CrowdWorldSubsystem.UpdateAureus` (subsystem `CrowdWorldSubsystem`) `Coin Increase`))

(fn `?KeepCoinsActive`
  (bind _returnvalue (`CrowdWorldSubsystem.KeepCoinsActive` (subsystem `CrowdWorldSubsystem`)))
  (if (and _returnvalue (`self.CoinsActive`))
    (`ActorComponent.Deactivate` (`Actor.RootComponent` (`self.CoinEffect`)))))

(fn `?LeaveCrowd`
  (returns (Leave :type Boolean))
  (locals (LeaveLikelihood :type "Float (double-precision)") (CrowdTimer :type "Float (double-precision)"))
  (if (> (`GameplayStatics.GetTimeSeconds`) (`local.CrowdTimer`))
    (set `local.CrowdTimer` (+ (`GameplayStatics.GetTimeSeconds`) 30.0))
    (bind _output_get (set `local.LeaveLikelihood` (/ 0.0 0.0)))
    (if (not (>= _output_get 0.2))
      (set `local.LeaveLikelihood` 0.2))
    (if (>= (`local.LeaveLikelihood`) (`KismetMathLibrary.RandomFloat`))
      (return false)
      (else
        (return true)))
    (else
      (`KismetSystemLibrary.PrintString` "false"))))

(fn `ThrowBall`
  (if (`self.CrowdPrime`)
    (`KismetSystemLibrary.PrintString` "Holding")
    (`/Game/BluePrints/InteractableSystem/BP_Spawn_Item.Spawn Thrown Item` (`self.Spawner`))
    (`CrowdWorldSubsystem.ResetExcitement` (subsystem `CrowdWorldSubsystem`))
    (set `self.itemcalled` false)
    (else
      (`KismetSystemLibrary.PrintString` "continue to cheer (handled by Audio Manager"))))

(fn `UpdateCrowd`
  (params (XP :type "Float (double-precision)"))
  (bind _returnvalue (subsystem `CrowdWorldSubsystem`))
  (bind _returnvalue_2 (+ (`CrowdWorldSubsystem.GetCrowdSize` _returnvalue) 5))
  (bind _returnvalue_3 (`CrowdWorldSubsystem.UpdateExcitement` (subsystem `CrowdWorldSubsystem`) XP))
  (`/Game/Audio/BP_AudioManager.Update Crowd Cheering` (`self.AudioManager`) _returnvalue_3)
  (`CrowdWorldSubsystem.SetCrowdSize` _returnvalue _returnvalue_2)
  (set `/Game/BluePrints/GlorySystem/CrowdVFX/BP_VFXCrowdController.CurrentCrowdSize` (`KismetMathLibrary.Conv_IntToDouble` _returnvalue_2) (`self.Crowd VFX Controller`)))

(fn `UserConstructionScript`)