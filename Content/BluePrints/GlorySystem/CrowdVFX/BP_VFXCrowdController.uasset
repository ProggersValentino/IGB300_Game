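; Glory system crowd VFX controller that switches the audience between sitting, standing and cheering effects and shows positive or negative emojis.
; ChangeCrowdVFX runs per-state timelines that blend MaskVis on the three crowd effects, though cheering zeroes sitting and leaves standing untouched.
; ActivateEmojis sets an emoji flag on the current state's effect, and a timeline clears all flags when finished.
; DetectExcitementLevel maps excitement to state names.
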(event `Activate Emojis`
  (params (IsGood :type Boolean))
  (`self.EmojiStates` IsGood)
  (`self.ResetEmojis`))

(event `ResetEmojis`
  (`Timeline|EmojiReset` :!via `PlayFromStart`
    (:`Finished`
      (`self.Deactivate Emojis`))))

(event `Change Crowd VFX`
  (params (StateName :type Name))
  (`|ExecutionSequence`
    (:`then_0`
      (switch `string` (`KismetStringLibrary.Conv_NameToString` StateName)
        (:`State_Sitting`
          (bind (_direction _gain _lose) (`Timeline|Timeline_1` :!via `PlayFromStart`)
            (:`Update`
              (set `self.CurrentSitMask` _gain)
              (set `self.CurrentStandMask` (* (`self.CurrentStandMask`) _lose))
              (set `self.CurrentCheerMask` (* (`self.CurrentCheerMask`) _lose))
              (`self.UpdateMasks`))))
        (:`State_Standing`
          (bind (_direction_2 _gain_2 _lose_2) (`Timeline|Timeline_0` :!via `PlayFromStart`)
            (:`Update`
              (set `self.CurrentSitMask` (* (`self.CurrentSitMask`) _lose_2))
              (set `self.CurrentStandMask` _gain_2)
              (set `self.CurrentCheerMask` (* (`self.CurrentCheerMask`) _lose_2))
              (`self.UpdateMasks`))))
        (:`State_Cheering`
          (bind (_direction_3 _gain_3) (`Timeline|Timeline` :!via `PlayFromStart`)
            (:`Update`
              (set `self.CurrentSitMask` (* (`self.CurrentSitMask`) 0.0))
              (set `self.CurrentCheerMask` _gain_3)
              (`self.UpdateMasks`))))))
    (:`then_1`
      (set `self.Current State Name` StateName))))

(fn `Deactivate Emojis`
  (bind _crowdsit (`self.CrowdSit`))
  (bind _crowdstand (`self.CrowdStand`))
  (bind _crowdcheer (`self.CrowdCheer`))
  (`|ExecutionSequence`
    (:`then_0`
      (`NiagaraComponent.SetVariableBool` _crowdsit "EmojiPos" false)
      (`NiagaraComponent.SetVariableBool` _crowdsit "EmojiNeg" false))
    (:`then_1`
      (`NiagaraComponent.SetVariableBool` _crowdstand "EmojiPos" false)
      (`NiagaraComponent.SetVariableBool` _crowdstand "EmojiNeg" false))
    (:`then_2`
      (`NiagaraComponent.SetVariableBool` _crowdcheer "EmojiPos" false)
      (`NiagaraComponent.SetVariableBool` _crowdcheer "EmojiNeg" false))))

(fn `DetectExcitementLevel`
  (params (Excitement :type "Float (double-precision)"))
  (returns (LevelKey :type String))
  (locals (StateIndex :type Integer))
  (set `local.StateIndex` (`KismetMathLibrary.FCeil` (- (/ (`KismetMathLibrary.FClamp` (* Excitement 4.0) 0.0 200.0) 99.0) 1.0)))
  (return (select `int` (`local.StateIndex`) :`0` "State_Sitting" :`1` "State_Standing" :`2` "State_Cheering" :`3` "NULL")))

(fn `EmojiStates`
  (params (Condition :type Boolean))
  (locals (BoolName :type Name :default "EmojiPos"))
  (bind _boolname (`local.BoolName`))
  (if Condition
    (set `local.BoolName` "EmojiPos")
    (else
      (set `local.BoolName` "EmojiNeg")))
  (switch `string` (`KismetStringLibrary.Conv_NameToString` (`self.Current State Name`))
    (:`State_Sitting`
      (`NiagaraComponent.SetVariableBool` (`self.CrowdSit`) _boolname true))
    (:`State_Standing`
      (`NiagaraComponent.SetVariableBool` (`self.CrowdStand`) _boolname true))
    (:`State_Cheering`
      (`NiagaraComponent.SetVariableBool` (`self.CrowdCheer`) _boolname true))))

(fn `UpdateMasks`
  (`NiagaraComponent.SetVariableFloat` (`self.CrowdSit`) "MaskVis" (`self.CurrentSitMask`))
  (`NiagaraComponent.SetVariableFloat` (`self.CrowdStand`) "MaskVis" (`self.CurrentStandMask`))
  (`NiagaraComponent.SetVariableFloat` (`self.CrowdCheer`) "MaskVis" (`self.CurrentCheerMask`)))

(fn `UserConstructionScript`)