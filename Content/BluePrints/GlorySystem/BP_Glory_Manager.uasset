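; Glory manager actor that tracks the gladiator player's XP and level, relaying glory changes to the crowd's excitement subsystem.
; ChangeXP adds a fixed amount; at MaxXP, IncreaseLevel spawns a random item through BP_Spawn_Item, without resetting XP.
; People'sMercy halves XP and applies a health-increase GameplayEffect when XP exceeds a cap, otherwise kills the player.
; BeginPlay caches actor references and runs a test Steam achievement write.
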(event `self.ReceiveBeginPlay`
  (bind _returnvalue (`GameplayStatics.GetPlayerController` 0))
  (`KismetSystemLibrary.DelayUntilNextTick`)
  (`|ExecutionSequence`
    (:`then_0`
      (bind _returnvalue_2 (`GameplayStatics.GetActorOfClass` "/Game/BluePrints/InteractableSystem/BP_Spawn_Item.BP_Spawn_Item_C"))
      (set `self.Spawner` _returnvalue_2)
      (bind _returnvalue_3 (`GameplayStatics.GetActorOfClass` "/Game/BluePrints/UI/HUDs/HBP_TestHUD_Attributes.HBP_TestHUD_Attributes_C"))
      (set `self.HUD` _returnvalue_3))
    (:`then_1`
      (bind _outactors (`GameplayStatics.GetAllActorsOfClass` "/Game/BluePrints/AI/CrowdAI/Crowd/BP_Crowd.BP_Crowd_C"))
      (set `self.Crowd` _outactors)
      (bind _returnvalue_4 (`GameplayStatics.GetActorOfClass` "/Game/BluePrints/Player/GladiatorRelated/BP_WWEGladiator_Player.BP_WWEGladiator_Player_C"))
      (set `self.Player Character BP` _returnvalue_4)
      ;[0.3538 0.7763 1] Steam Achievment Test
      (`AchievementQueryCallbackProxy.CacheAchievements` _returnvalue
        (:`then`
          (`KismetSystemLibrary.PrintString` "attempt to get achievement" false))
        (:`OnSuccess`
          (`AchievementWriteCallbackProxy.WriteAchievementProgress` _returnvalue "TestAchievement" 1.0))
        (:`OnFailure`
          (`KismetSystemLibrary.PrintString` "failed to get achievement" false))))))

(event `People's Mercy`
  (if (> (`self.XP`) (`self.PeoplesMercyCap`))
    (bind _output_get (set `self.XP` (/ (`self.XP`) 2.0)))
    (`CrowdWorldSubsystem.UpdateExcitement` (subsystem `CrowdWorldSubsystem`) _output_get)
    (`AbilitySystemComponent.BP_ApplyGameplayEffectToTarget` :`self` (`AbilitySystemBlueprintLibrary.GetAbilitySystemComponent` (`self.Player Character BP`)) :`GameplayEffectClass` "/Game/BluePrints/InteractableSystem/GameEffects/GE_Item_HealthIncrease.GE_Item_HealthIncrease_C")
    (else
      (`/Game/BluePrints/Player/GladiatorRelated/BP_WWEGladiator_Player.Death` (`self.Player Character BP`)))))

(fn `(Deprecated)DetermineItem`
  (returns (Item :type "/Game/BluePrints/InteractableSystem/Interactable Class Reference"))
  (return (`KismetArrayLibrary.Array_Random` (`self.Item`))))

(fn `(Deprecated)Increase Level`
  (params (`Added Level` :type Integer))
  (set `self.Level` (+ (`self.Level`) `Added Level`))
  (`TextBlock.SetText` (`/Game/BluePrints/UI/Widgets/OldWidgets/Widget_HUD.LevelTxt` (`/Game/BluePrints/UI/HUDs/HBP_TestHUD_Attributes.UI_Ref` (`self.HUD`))) (`KismetTextLibrary.Conv_IntToText` (`self.Level`)))
  (bind _item (`self.(Deprecated)DetermineItem`))
  (`/Game/BluePrints/InteractableSystem/BP_Spawn_Item.SpawnItem` (`self.Spawner`) _item (0.0 0.0 0.0)))

(fn `Change XP`
  (params (`Added XP` :type "Float (double-precision)"))
  (bind _output_get (set `self.Added XP` 10.0))
  (`|ExecutionSequence`
    (:`then_0`
      ;[1 1 1] Relay info to Crowd
      (`CrowdWorldSubsystem.UpdateExcitement` (subsystem `CrowdWorldSubsystem`) _output_get))
    (:`then_1`
      ;[1 1 1] Update XP and Level Variable
      (set `self.XP` (+ (`self.XP`) 10.0))
      (if (>= (`self.XP`) (`self.Max XP`))
        (`self.IncreaseLevel` 0)))))

(fn `IncreaseLevel`
  (params (AddLevel :type Integer))
  (returns (ReturnValue :type Boolean))
  (set `self.Level` (+ (`self.Level`) AddLevel))
  (bind _item (`self.(Deprecated)DetermineItem`))
  (`/Game/BluePrints/InteractableSystem/BP_Spawn_Item.SpawnItem` (`self.Spawner`) _item (0.0 0.0 0.0))
  (return false))

(fn `ResetGlory`
  (params (`XP Value` :type "Float (double-precision)") (`Level Value` :type Integer))
  (set `self.XP` `XP Value`)
  (set `self.Level` `Level Value`))

(fn `UserConstructionScript`)