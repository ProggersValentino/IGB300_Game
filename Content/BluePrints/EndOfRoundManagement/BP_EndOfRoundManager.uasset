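; End-of-round manager actor that runs the between-round sequence and grants achievements.
; EndOfRoundStuff increments the round counter, shows the WB_EndScreen widget and grows the crowd through CrowdWorldSubsystem.
; At round five it caches achievements and writes Champion, plus BloodBath for enough blood spilled or otherwise CrowdWeezer for no cumulative excitement, skipping completed ones.
; BeginPlay finds BP_EnemyManager after a race-avoiding delay, but that reference is unused and the binding call is disconnected.
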(event `self.ReceiveBeginPlay`
  (`KismetSystemLibrary.Delay` 0.2) ; prevent from a race condition bug
  (bind _returnvalue (`GameplayStatics.GetActorOfClass` "/Game/BluePrints/AI/EnemyRelated/BP_EnemyManager.BP_EnemyManager_C"))
  (set `self.WaveManager` _returnvalue))

(event `EndOfRoundStuff`
  (bind _returnvalue (`GameplayStatics.GetPlayerController` 0))
  (bind _returnvalue_2 (`GameplayStatics.GetPlayerController` 0))
  (bind _returnvalue_3 (`GameplayStatics.GetPlayerController` 0))
  (bind _returnvalue_4 (subsystem `CrowdWorldSubsystem`))
  (`KismetSystemLibrary.PrintString` "End of round stuff")
  (set `self.RoundCounter` (+ (`self.RoundCounter`) 1))
  (bind _returnvalue_5 (`|CreateWidget` "/Game/BluePrints/UI/EndScreen/WB_EndScreen.WB_EndScreen_C" (`GameplayStatics.GetPlayerController` 0)))
  (bind _output_get (set `self.endOfRoundWidget` _returnvalue_5))
  (`UserWidget.AddToViewport` _output_get 0)
  (`CrowdWorldSubsystem.SetCrowdSize` _returnvalue_4 (+ (`CrowdWorldSubsystem.GetCrowdSize` _returnvalue_4) 50))
  ;[1 1 1] Reward Champion
  (if (== (`self.RoundCounter`) 5)
    (`AchievementQueryCallbackProxy.CacheAchievements` _returnvalue_3
      (:`then`
        ;[1 1 1] Reward Bloodbath
        (if (>= (`GameplayStats.GetBloodSpilled` (subsystem `GameplayStats`)) 1000.0)
          (`AchievementQueryCallbackProxy.CacheAchievements` _returnvalue_2
            (:`OnSuccess`
              (bind (_bfoundid _progress) (`AchievementBlueprintLibrary.GetCachedAchievementProgress` _returnvalue_2 "BloodBath"))
              (if (not (== _progress 1.0))
                (`AchievementWriteCallbackProxy.WriteAchievementProgress` _returnvalue_2 "BloodBath" 1.0))))
          (else
            ;[1 1 1] Reward CrowdWeezer
            (if (<= (`CrowdWorldSubsystem.GetCumulativeExcitement` (subsystem `CrowdWorldSubsystem`)) 0.0)
              (`AchievementQueryCallbackProxy.CacheAchievements` _returnvalue
                (:`OnSuccess`
                  (bind (_bfoundid_2 _progress_2) (`AchievementBlueprintLibrary.GetCachedAchievementProgress` _returnvalue "CrowdWeezer"))
                  (if (not (== _progress_2 1.0))
                    (`AchievementWriteCallbackProxy.WriteAchievementProgress` _returnvalue "CrowdWeezer" 1.0))))))))
      (:`OnSuccess`
        (bind (_bfoundid_3 _progress_3) (`AchievementBlueprintLibrary.GetCachedAchievementProgress` _returnvalue_3 "Champion"))
        (if (not (== _progress_3 1.0))
          (`AchievementWriteCallbackProxy.WriteAchievementProgress` _returnvalue_3 "Champion" 1.0))))))

(fn `UserConstructionScript`)