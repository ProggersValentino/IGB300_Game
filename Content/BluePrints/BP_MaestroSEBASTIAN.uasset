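; BP_MaestroSEBASTIAN is the round manager for the gladiator game, running five rounds of melee enemy waves to a win screen.
; Tick detects the last enemy's death, then timelines spin the camera and fade a post-process material fed by player scene captures, frozen for the final-kill shot.
; A random sequence and end-of-round widget follow, crowd size grows, and round five awards achievements.
; NextRound restores camera and captures, then spawns enemies or shows victory.
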(event `self.ReceiveTick`
  (params (DeltaSeconds :type "Float (single-precision)"))
  (bind _outactors (`GameplayStatics.GetAllActorsOfClass` "/Game/BluePrints/AI/EnemyRelated/Enemies/BP_BasicMeleeEnemy.BP_BasicMeleeEnemy_C"))
  (if (<= (`KismetArrayLibrary.Array_Length` _outactors) 1)
    (for _array_element _outactors
      (if (and (`/Game/BluePrints/AI/EnemyRelated/Enemies/BP_BasicMeleeEnemy.IsDead` _array_element) (== (`self.State`) "Round"))
        (`self.BeginEndOfRound`)
        (`self.SetActorTickEnabled` false)))))

(event `self.ReceiveBeginPlay`
  (bind _asbp_wwegladiator_player (cast `/Game/BluePrints/Player/GladiatorRelated/BP_WWEGladiator_Player` (`GameplayStatics.GetPlayerCharacter` 0))
    (:`then`
      (set `self.Player` _asbp_wwegladiator_player)
      (`self.ScreenSetup`)
      (`self.Final Kill PPSetup`)
      (bind _returnvalue (`GameplayStatics.GetActorOfClass` "/Game/Audio/BP_AudioManager.BP_AudioManager_C"))
      (set `self.AudioManager` _returnvalue)
      (`self.NextRound`))
    (:`CastFailed`
      (`KismetSystemLibrary.PrintString` "NO PLAYER"))))

(event `BeginEndOfRound`
  (bind _returnvalue (`GameplayStatics.GetPlayerController` 0))
  (bind _returnvalue_2 (`GameplayStatics.GetPlayerController` 0))
  (bind _returnvalue_3 (`GameplayStatics.GetPlayerController` 0))
  (bind _returnvalue_4 (subsystem `CrowdWorldSubsystem`))
  (bind _endofroundwidget (`self.endOfRoundWidget`))
  (bind _returnvalue_5 (+ (`CrowdWorldSubsystem.GetCrowdSize` _returnvalue_4) 100))
  (set `self.State` "EndRound")
  (`self.Toggle Camera` false)
  (bind (_direction _yaw) (`Timeline|CameraYaw`)
    (:`Update`
      (`SceneComponent.K2_SetRelativeRotation` (`/Game/BluePrints/Player/GladiatorRelated/BP_WWEGladiator_Player.CameraBoom` (`self.Player`)) (`KismetMathLibrary.MakeRotator` 0.0 0.0 (+ _yaw (`self.CurrentCameraYaw`))) false false))
    (:`Finished`
      (`self.Toggle Captures` false)
      (`/Game/Audio/BP_AudioManager.UpdateCrowdVolume` (`self.AudioManager`) true)
      (bind (_direction_2 _fade) (`Timeline|FinishFade`)
        (:`Update`
          (`MaterialInstanceDynamic.SetScalarParameterValue` (`self.ScreenRenderMaterial`) "FadeEnd" _fade))
        (:`Finished`
          (`KismetSystemLibrary.Delay` 1.0)
          (`self.StartSequence` (`KismetArrayLibrary.Array_Random` (`self.EndRoundSequences`)))
          (set `self.RoundCounter` (+ (`self.RoundCounter`) 1))
          (`/Game/BluePrints/UI/EndScreen/WB_EndScreen.Now Open` _endofroundwidget)
          (`Widget.SetVisibility` _endofroundwidget "Visible")
          (`CrowdWorldSubsystem.SetCrowdSize` _returnvalue_4 _returnvalue_5)
          (bind _returnvalue_6 (`GameplayStatics.GetActorOfClass` "/Game/BluePrints/GlorySystem/CrowdVFX/BP_VFXCrowdController.BP_VFXCrowdController_C"))
          ;[1 1 1] Reward Champion
          (set `/Game/BluePrints/GlorySystem/CrowdVFX/BP_VFXCrowdController.CurrentCrowdSize` (`KismetMathLibrary.Conv_IntToDouble` _returnvalue_5) _returnvalue_6)
          (if (== (`self.RoundCounter`) 5)
            (`AchievementQueryCallbackProxy.CacheAchievements` _returnvalue_3
              (:`then`
                ;[1 1 1] Reward Bloodbath
                (if (>= (`GameplayStats.GetBloodSpilled` (subsystem `GameplayStats`)) 1000.0)
                  (`AchievementQueryCallbackProxy.CacheAchievements` _returnvalue_2
                    (:`OnSuccess`
                      (bind (_bfoundid _progress) (`AchievementBlueprintLibrary.GetCachedAchievementProgress` _returnvalue_2 "BloodBath"))
                      (if (not (== _progress 1.0))
                        (`AchievementWriteCallbackProxy.WriteAchievementProgress` _returnvalue_2 "BloodBath" 1.0))))
                  (else
                    ;[1 1 1] Reward CrowdWeezer
                    (if (<= (`CrowdWorldSubsystem.GetCumulativeExcitement` (subsystem `CrowdWorldSubsystem`)) 0.0)
                      (`AchievementQueryCallbackProxy.CacheAchievements` _returnvalue
                        (:`OnSuccess`
                          (bind (_bfoundid_2 _progress_2) (`AchievementBlueprintLibrary.GetCachedAchievementProgress` _returnvalue "CrowdWeezer"))
                          (if (not (== _progress_2 1.0))
                            (`AchievementWriteCallbackProxy.WriteAchievementProgress` _returnvalue "CrowdWeezer" 1.0))))))))
              (:`OnSuccess`
                (bind (_bfoundid_3 _progress_3) (`AchievementBlueprintLibrary.GetCachedAchievementProgress` _returnvalue_3 "Champion"))
                (if (not (== _progress_3 1.0))
                  (`AchievementWriteCallbackProxy.WriteAchievementProgress` _returnvalue_3 "Champion" 1.0))))))))))

(event `NextRound`
  (bind _returnvalue (`GameplayStatics.GetPlayerController` 0))
  (bind (_returnvalue_x _returnvalue_y) (`KismetMathLibrary.BreakVector2D` (`WidgetLayoutLibrary.GetViewportSize`)))
  (`MaterialInstanceDynamic.SetScalarParameterValue` (`self.ScreenRenderMaterial`) "FadeEnd" 0.0)
  (`self.Toggle Camera` true)
  (`self.Toggle Captures` true)
  (`/Game/Audio/BP_AudioManager.UpdateCrowdVolume` (`self.AudioManager`) false)
  (`/Game/BluePrints/UI/WP_ScreenWipe.FadeOut` (`self.ScreenWipe`))
  (if (>= (`self.RoundCounter`) 5)
    (bind _returnvalue_2 (`|CreateWidget` "/Game/BluePrints/UI/Widgets/WBP_DeathUI.WBP_DeathUI_C" (`GameplayStatics.GetPlayerController` 0)))
    (set `TextBlock.Text` "You Won!" (`/Game/BluePrints/UI/Widgets/WBP_DeathUI.Lost_Base` _returnvalue_2))
    (set `TextBlock.Text` "You Won!" (`/Game/BluePrints/UI/Widgets/WBP_DeathUI.Lost_Shadow` _returnvalue_2))
    (`UserWidget.AddToViewport` _returnvalue_2 0)
    (`WidgetBlueprintLibrary.SetInputMode_GameAndUIEx` _returnvalue _returnvalue_2 "LockInFullscreen")
    (set `PlayerController.bShowMouseCursor` true _returnvalue)
    (`GameplayStatics.SetGamePaused` true)
    (`PlayerController.SetMouseLocation` _returnvalue (`KismetMathLibrary.FTrunc` (/ _returnvalue_x 2.0)) (`KismetMathLibrary.FTrunc` (/ _returnvalue_y 2.0)))
    (else
      (set `self.State` "Round")
      (`EnemySubsystem.TrySpawn` (subsystem `EnemySubsystem`) "NORMAL" "/Game/BluePrints/AI/EnemyRelated/Enemies/BP_BasicMeleeEnemy.BP_BasicMeleeEnemy_C")
      (`self.SetActorTickEnabled` true))))

(event `StartSequence`
  (params (Sequence :type "LevelSequenceActor Object Reference"))
  (bind _sequenceplayer (`LevelSequenceActor.SequencePlayer` Sequence))
  (bind _player (`self.Player`))
  (`/Game/BluePrints/UI/WP_ScreenWipe.FadeOut` (`self.ScreenWipe`))
  (`/Engine/EditorBlueprintResources/StandardMacros.IsValid` Sequence
    (:`Is Valid`
      (`MovieSceneSequencePlayer.Play` _sequenceplayer)
      (`self.DisableInput` _player null)
      (`KismetSystemLibrary.Delay` (`TimeManagementBlueprintLibrary.Conv_QualifiedFrameTimeToSeconds` (`MovieSceneSequencePlayer.GetDuration` _sequenceplayer)))
      (`self.EnableInput` _player null))))

(fn `Final Kill PPSetup`
  (locals (NewLocalVar :type "Array of PostProcessSettings Structure"))
  (bind _returnvalue (`KismetMaterialLibrary.CreateDynamicMaterialInstance` "/Game/BluePrints/UI/RenderCapture/RT_EndScreenCapture_Mat.RT_EndScreenCapture_Mat" "RenderScreenTest"))
  (bind _output_get (set `self.ScreenRenderMaterial` _returnvalue))
  (`MaterialInstanceDynamic.SetScalarParameterValue` _output_get "FadeEnd" 0.0)
  (setmembers `PostProcessSettings` :`StructRef` (`CameraComponent.PostProcessSettings` (`/Game/BluePrints/Player/GladiatorRelated/BP_WWEGladiator_Player.FollowCamera` (`self.Player`))) :`WeightedBlendables` (make `WeightedBlendables` (`|MakeArray` (make `WeightedBlendable` 1.0 _output_get)))))

(fn `ScreenSetup`
  (bind _returnvalue (`GameplayStatics.GetPlayerController` 0))
  (`|ExecutionSequence`
    (:`then_0`
      (bind _returnvalue_2 (`|CreateWidget` "/Game/BluePrints/UI/EndScreen/WB_EndScreen.WB_EndScreen_C" _returnvalue))
      (bind _output_get (set `self.endOfRoundWidget` _returnvalue_2))
      (`Widget.SetVisibility` _output_get "Hidden")
      (`UserWidget.AddToViewport` _output_get 0))
    (:`then_1`
      (bind _returnvalue_3 (`|CreateWidget` "/Game/BluePrints/UI/WP_LoadingScreen.WP_LoadingScreen_C" _returnvalue))
      (bind _output_get_2 (set `self.LoadingScreen` _returnvalue_3))
      (`Widget.SetVisibility` _output_get_2 "Hidden")
      (`UserWidget.AddToViewport` _output_get_2 0))
    (:`then_2`
      (bind _returnvalue_4 (`|CreateWidget` "/Game/BluePrints/UI/WP_ScreenWipe.WP_ScreenWipe_C" _returnvalue))
      (bind _output_get_3 (set `self.ScreenWipe` _returnvalue_4))
      (`UserWidget.AddToViewport` _output_get_3 0))))

(fn `Toggle Camera`
  (params (Toggle :type Boolean))
  (bind _returnvalue (`GameplayStatics.GetPlayerController` 0))
  (bind _player (`self.Player`))
  (bind _cameraboom (`/Game/BluePrints/Player/GladiatorRelated/BP_WWEGladiator_Player.CameraBoom` (`self.Player`)))
  (bind (_relativerotation_roll _relativerotation_pitch) (`KismetMathLibrary.BreakRotator` (`SceneComponent.RelativeRotation` _cameraboom)))
  (set `GladiatorPlayerChar.bUseCameraLerpWithMouse` Toggle (`self.Player`))
  (set `SpringArmComponent.bInheritYaw` Toggle _cameraboom)
  (if Toggle
    (`self.EnableInput` _player _returnvalue)
    (else
      (`self.DisableInput` _player _returnvalue)
      (set `self.CurrentCameraYaw` _relativerotation_pitch))))

(fn `Toggle Captures`
  (params (Toggle :type Boolean))
  (bind _player (`self.Player`))
  (set `SceneCaptureComponent.bCaptureEveryFrame` Toggle (`/Game/BluePrints/Player/GladiatorRelated/BP_WWEGladiator_Player.BaseCapture` _player))
  (set `SceneCaptureComponent.bCaptureEveryFrame` Toggle (`/Game/BluePrints/Player/GladiatorRelated/BP_WWEGladiator_Player.FinisherCapture` _player)))

(fn `UserConstructionScript`)